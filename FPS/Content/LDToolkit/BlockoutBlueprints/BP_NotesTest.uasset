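; BP_NotesTest is a level-design blockout note actor that shows text on a backing cube, with a pointer line to an offset location.
; The construction script applies the note text and size, then scales and positions the cube from the rendered text bounds.
; It moves a sphere to MeasureLocation and centers, rotates and stretches a cylinder between the origin and that point, using the offset's length.
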(fn ConstructionScript
  (bind _textrender (Variables|Default|GetTextRender))
  (bind _cube (Variables|Default|GetCube))
  (bind _returnvalue (Class|TextRenderComponent|GetTextLocalSize _textrender))
  (bind _returnvalue_2 (Transformation|GetWorldScale _cube))
  (|CallParentFunction)
  ;[1 1 1] Set Text Size
  (Rendering|Components|TextRender|SetWorldSize (Variables|Default|GetTextRender) (Variables|Default|GetTextSize))
  ;[1 1 1] Set the text based on the variable
  (Rendering|Components|TextRender|SetText (Variables|Default|GetTextRender) (Variables|Default|GetNoteText))
  ;[1 1 1] Set scale of the background cube based on the text size
  (Transformation|SetWorldScale3D (Variables|Default|GetCube) (Math|Vector|MakeVector 0.05 (+ (/ (.y _returnvalue) 1e+02) 0.2) (+ (/ (.z _returnvalue) 1e+02) 0.2)))
  ;[1 1 1] Set the location of the background cube
  (Transformation|SetRelativeLocation (Variables|Default|GetCube) (Math|Vector|MakeVector -0.025 (* (/ (.y _returnvalue_2) 2.0) -1e+02) (* (/ (.z _returnvalue_2) 2.0) 1e+02)) false false)
  ;[1 1 1] Sets Sphere at the end point
  (Transformation|SetRelativeLocation (Variables|Default|GetSphere1) (Variables|Default|GetMeasure%20Location) false false)
  ;[1 1 1] Sets the cylinder between the two spheres
  (Transformation|SetRelativeLocation (Variables|Default|GetScene) (/ (Variables|Default|GetMeasure%20Location) 2) false false)
  ;[1 1 1] Sets the rotation of the cylinder to point between the two sphere
  (Transformation|SetRelativeRotation (Variables|Default|GetScene) (Math|Rotator|FindLookatRotation (Math|Vector|MakeVector 0.0 0.0 0.0) (Variables|Default|GetMeasure%20Location)) false false)
  ;[1 1 1] Set cylinder scale to fit between the two spheres
  (Transformation|SetRelativeScale3D (Variables|Default|GetCylinder) (Math|Vector|MakeVector 0.05 0.05 (|Findthehypotenuse_2_2))))