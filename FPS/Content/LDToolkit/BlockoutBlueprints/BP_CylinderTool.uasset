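; BP_CylinderTool is a level-design blockout actor that builds a full, half or quarter cylinder shaped by a 3D widget point, Corner.
; The construction script picks the mesh from the CylinderType enum and applies the chosen Material.
; Corner's XY length sets the radial scale and its direction sets the yaw, offset by 90 degrees.
; Corner's Z drives the height scale and raises the mesh by half that value.
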(event EventBeginPlay)

(event Collision|EventActorBeginOverlap
  (params (OtherActor :type Actor%20Object%20Reference)))

(event EventTick
  (params (DeltaSeconds :type Float%20%28single-precision%29)))

(fn ConstructionScript
  (bind _returnvalue (Math|Vector|MakeVector 0.0 0.0 0.0))
  (bind _corner (Variables|Default|GetCorner))
  (bind _corner_2 (Variables|Default|GetCorner))
  (bind _returnvalue_2 (Math|Vector|MakeVector (.x _corner) (.y _corner) 0.0))
  (bind _returnvalue_3 (/ _corner_2 100))
  (bind _returnvalue_4 (Math|Rotator|FindLookatRotation _returnvalue _returnvalue_2))
  (bind _returnvalue_5 (Math|Vector|MakeVector (.x _returnvalue_3) (.y _returnvalue_3) 0.0))
  (bind _returnvalue_6 (Math|Vector|VectorLength _returnvalue_5))
  ;[1 1 1] Sets the scale of the static mesh based on the 3D Widget
  (Transformation|SetWorldScale3D (Variables|Default|GetStaticMesh) (Math|Vector|MakeVector _returnvalue_6 _returnvalue_6 (/ (.z _returnvalue_3) 2.0)))
  ;[1 1 1] Sets the static mesh based on the Enum
  (Components|StaticMesh|SetStaticMesh (Variables|Default|GetStaticMesh) (Utilities|Select :Index (Variables|Default|GetCylinderType) :NewEnumerator0 "/Game/LDToolkit/Back-end/Models/SM_CylinderTool.SM_CylinderTool" :NewEnumerator1 "/Game/LDToolkit/Back-end/Models/SM_HalfCylinderTool.SM_HalfCylinderTool" :NewEnumerator2 "/Game/LDToolkit/Back-end/Models/SM_QuarterCylinderTool.SM_QuarterCylinderTool"))
  ;[1 1 1] Sets the rotation of the static mesh to fit the 3D Widget
  (Transformation|SetRelativeRotation (Variables|Default|GetStaticMesh) (Math|Rotator|MakeRotator (.roll _returnvalue_4) (.pitch _returnvalue_4) (+ (.yaw _returnvalue_4) 9e+01)) false false)
  ;[1 1 1] Sets the location of the cylinder based on the 3D Widget
  (Transformation|SetRelativeLocation (Variables|Default|GetStaticMesh) (Math|Vector|MakeVector 0.0 0.0 (/ (.z (Variables|Default|GetCorner)) 2.0)) false false)
  ;[1 1 1] Set the material of the static mesh
  (Rendering|Material|SetMaterial (Variables|Default|GetStaticMesh) 0 (Variables|Default|GetMaterial)))