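; Blockout vent intersection for level design: a resizable hollow box with side walls that can be opened individually.
; The construction script scales and positions top, bottom, four corner posts and four side panels from the Corner vector and OuterThickness, keeping the origin at one bottom corner.
; Per-side booleans toggle each panel's visibility and collision together.
; All pieces share the MainColor material.
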(fn ConstructionScript
  (bind _corner (Variables|Default|GetCorner))
  (bind _corner_2 (Variables|Default|GetCorner))
  (bind _corner_3 (Variables|Default|GetCorner))
  (bind _outer_thickness (Variables|Default|GetOuter%20Thickness))
  (bind _corner_4 (Variables|Default|GetCorner))
  (bind _corner_5 (Variables|Default|GetCorner))
  (bind _corner_6 (Variables|Default|GetCorner))
  (bind _outer_thickness_2 (Variables|Default|GetOuter%20Thickness))
  (bind _corner_7 (Variables|Default|GetCorner))
  (bind _outer_thickness_3 (Variables|Default|GetOuter%20Thickness))
  (bind _corner_8 (Variables|Default|GetCorner))
  (bind _corner_9 (Variables|Default|GetCorner))
  (bind _corner_10 (Variables|Default|GetCorner))
  (bind _corner_11 (Variables|Default|GetCorner))
  (bind _corner_12 (Variables|Default|GetCorner))
  (bind _outer_thickness_4 (Variables|Default|GetOuter%20Thickness))
  (bind _corner_13 (Variables|Default|GetCorner))
  (bind _corner_14 (Variables|Default|GetCorner))
  (bind _outer_thickness_5 (Variables|Default|GetOuter%20Thickness))
  (bind _corner_15 (Variables|Default|GetCorner))
  (bind _outer_thickness_6 (Variables|Default|GetOuter%20Thickness))
  (bind _returnvalue (* _outer_thickness_2 5e+01))
  (bind _returnvalue_2 (* _outer_thickness_3 5e+01))
  (bind _returnvalue_3 (* _outer_thickness_4 2.0))
  (bind _returnvalue_4 (* _outer_thickness_5 2.0))
  (bind _returnvalue_5 (* _outer_thickness_6 2.0))
  (bind _returnvalue_6 (* _outer_thickness 2.0))
  (|CallParentFunction)
  (Rendering|Material|SetMaterial (Variables|Default|Get4) 0 (Variables|Default|GetMain%20Color))
  (Rendering|Material|SetMaterial (Variables|Default|Get3) 0 (Variables|Default|GetMain%20Color))
  (Rendering|Material|SetMaterial (Variables|Default|Get2) 0 (Variables|Default|GetMain%20Color))
  (Rendering|Material|SetMaterial (Variables|Default|Get1) 0 (Variables|Default|GetMain%20Color))
  (Rendering|Material|SetMaterial (Variables|Default|GetBottom) 0 (Variables|Default|GetMain%20Color))
  (Rendering|Material|SetMaterial (Variables|Default|GetTop) 0 (Variables|Default|GetMain%20Color))
  (Transformation|SetRelativeScale3D (Variables|Default|GetTop) (Math|Vector|MakeVector (/ (.x _corner_10) 1e+02) (/ (.y _corner_10) 1e+02) (Variables|Default|GetOuter%20Thickness)))
  (Transformation|SetRelativeLocation (Variables|Default|GetTop) (Math|Vector|MakeVector (/ (.x _corner_2) 2.0) (/ (.y _corner_2) 2.0) (- (.z (Variables|Default|GetCorner)) (* (Variables|Default|GetOuter%20Thickness) 5e+01))) false false)
  (Transformation|SetRelativeScale3D (Variables|Default|GetBottom) (Math|Vector|MakeVector (/ (.x _corner_5) 1e+02) (/ (.y _corner_5) 1e+02) (Variables|Default|GetOuter%20Thickness)))
  (Transformation|SetRelativeLocation (Variables|Default|GetBottom) (Math|Vector|MakeVector (/ (.x _corner) 2.0) (/ (.y _corner) 2.0) (* (Variables|Default|GetOuter%20Thickness) 5e+01)) false false)
  (CallFunction|SetCornerSizes (Variables|Default|Get1))
  (CallFunction|SetCornerSizes (Variables|Default|Get2))
  (CallFunction|SetCornerSizes (Variables|Default|Get3))
  (CallFunction|SetCornerSizes (Variables|Default|Get4))
  (Transformation|SetRelativeLocation (Variables|Default|Get2) (Math|Vector|MakeVector (- (.x _corner_6) _returnvalue) (- (.y _corner_6) _returnvalue) (/ (.z _corner_6) 2.0)) false false)
  (Transformation|SetRelativeLocation (Variables|Default|Get1) (Math|Vector|MakeVector (- (.x _corner_9) (* (Variables|Default|GetOuter%20Thickness) 5e+01)) (* (Variables|Default|GetOuter%20Thickness) 5e+01) (/ (.z _corner_9) 2.0)) false false)
  (Transformation|SetRelativeLocation (Variables|Default|Get3) (Math|Vector|MakeVector (* (Variables|Default|GetOuter%20Thickness) 5e+01) (- (.y _corner_8) (* (Variables|Default|GetOuter%20Thickness) 5e+01)) (/ (.z _corner_8) 2.0)) false false)
  (Transformation|SetRelativeLocation (Variables|Default|Get4) (Math|Vector|MakeVector _returnvalue_2 _returnvalue_2 (/ (.z (Variables|Default|GetCorner)) 2.0)) false false)
  (CallFunction|SetVisibilityandCollision (Variables|Default|GetFront) (Variables|Default|GetShow%20Front%20Side))
  (CallFunction|SetVisibilityandCollision (Variables|Default|GetBack) (Variables|Default|GetShow%20Back%20Side))
  (CallFunction|SetVisibilityandCollision (Variables|Default|GetRight) (Variables|Default|GetShow%20Right%20Side))
  (CallFunction|SetVisibilityandCollision (Variables|Default|GetLeft) (Variables|Default|GetShow%20Left%20Side))
  (Transformation|SetRelativeLocation (Variables|Default|GetFront) (Math|Vector|MakeVector (/ (.x _corner_11) 2.0) (- (.y _corner_11) (* (Variables|Default|GetOuter%20Thickness) 5e+01)) (/ (.z _corner_11) 2.0)) false false)
  (Transformation|SetRelativeScale3D (Variables|Default|GetFront) (Math|Vector|MakeVector (- (/ (.x _corner_12) 1e+02) _returnvalue_3) (Variables|Default|GetOuter%20Thickness) (- (/ (.z _corner_12) 1e+02) _returnvalue_3)))
  (Transformation|SetRelativeLocation (Variables|Default|GetBack) (Math|Vector|MakeVector (/ (.x _corner_13) 2.0) (* (Variables|Default|GetOuter%20Thickness) 5e+01) (/ (.z _corner_13) 2.0)) false false)
  (Transformation|SetRelativeScale3D (Variables|Default|GetBack) (Math|Vector|MakeVector (- (/ (.x _corner_15) 1e+02) _returnvalue_5) (Variables|Default|GetOuter%20Thickness) (- (/ (.z _corner_15) 1e+02) _returnvalue_5)))
  (Transformation|SetRelativeLocation (Variables|Default|GetRight) (Math|Vector|MakeVector (* (Variables|Default|GetOuter%20Thickness) 5e+01) (/ (.y _corner_4) 2.0) (/ (.z _corner_4) 2.0)) false false)
  (Transformation|SetRelativeScale3D (Variables|Default|GetRight) (Math|Vector|MakeVector (Variables|Default|GetOuter%20Thickness) (- (/ (.y _corner_14) 1e+02) _returnvalue_4) (- (/ (.z _corner_14) 1e+02) _returnvalue_4)))
  (Transformation|SetRelativeLocation (Variables|Default|GetLeft) (Math|Vector|MakeVector (- (.x _corner_7) (* (Variables|Default|GetOuter%20Thickness) 5e+01)) (/ (.y _corner_7) 2.0) (/ (.z _corner_7) 2.0)) false false)
  (Transformation|SetRelativeScale3D (Variables|Default|GetLeft) (Math|Vector|MakeVector (Variables|Default|GetOuter%20Thickness) (- (/ (.y _corner_3) 1e+02) _returnvalue_6) (- (/ (.z _corner_3) 1e+02) _returnvalue_6)))
  (Rendering|Material|SetMaterial (Variables|Default|GetFront) 0 (Variables|Default|GetMain%20Color))
  (Rendering|Material|SetMaterial (Variables|Default|GetBack) 0 (Variables|Default|GetMain%20Color))
  (Rendering|Material|SetMaterial (Variables|Default|GetLeft) 0 (Variables|Default|GetMain%20Color))
  (Rendering|Material|SetMaterial (Variables|Default|GetRight) 0 (Variables|Default|GetMain%20Color)))

(fn SetCornerSizes
  (params (Corner%20Piece :type Scene%20Component%20Object%20Reference))
  (bind _outer_thickness (Variables|Default|GetOuter%20Thickness))
  (Transformation|SetRelativeScale3D Corner%20Piece (Math|Vector|MakeVector _outer_thickness _outer_thickness (- (/ (.z (Variables|Default|GetCorner)) 1e+02) (* (Variables|Default|GetOuter%20Thickness) 2.0)))))

(fn SetVisibilityandCollision
  (params (Side :type Static%20Mesh%20Component%20Object%20Reference) (IsVisible :type Boolean))
  (Rendering|SetVisibility Side IsVisible false)
  (Collision|SetCollisionEnabled Side (select IsVisible "QueryAndPhysics" "NoCollision")))