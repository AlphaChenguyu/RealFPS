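; Level-design blockout actor for pipe junctions, switchable between 90-degree corner, 45-degree corner, 3-way and 4-way intersection.
; The construction script scales and offsets five pipe components from the Corner vector, swapping X and Z scale on the side pipes.
; PipeType selects which components are visible.
; MainColor is applied only to the straight and side pipes, not the corner pieces.
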(event EventBeginPlay
  (|CallParentFunction) ; This node is disabled and will not be called.\nDrag off pins to build functionality.
)

(event Collision|EventActorBeginOverlap
  (params (OtherActor :type Actor%20Object%20Reference))
  (|CallParentFunction OtherActor) ; This node is disabled and will not be called.\nDrag off pins to build functionality.
)

(event EventTick
  (params (DeltaSeconds :type Float%20%28single-precision%29))
  (|CallParentFunction DeltaSeconds) ; This node is disabled and will not be called.\nDrag off pins to build functionality.
)

(fn ConstructionScript
  (bind _corner (Variables|Default|GetCorner))
  (bind _corner_2 (Variables|Default|GetCorner))
  (bind _corner_3 (Variables|Default|GetCorner))
  (bind _corner_4 (Variables|Default|GetCorner))
  (bind _returnvalue (/ _corner_2 2))
  (bind _returnvalue_2 (/ _corner_4 50))
  (bind _returnvalue_3 (/ _corner 50))
  (bind _returnvalue_4 (/ _corner_3 2))
  (|CallParentFunction)
  (Utilities|FlowControl|Sequence
    (:then_0
      ;[1 1 1] Set the scale of the box based on the corner variable
      (Transformation|SetWorldScale3D (Variables|Default|GetPipe%20Straight) (/ (Variables|Default|GetCorner) 50))
      (Transformation|SetWorldScale3D (Variables|Default|GetPipe%20Side%201) (Math|Vector|MakeVector (.z _returnvalue_2) (.y _returnvalue_2) (.x _returnvalue_2)))
      (Transformation|SetWorldScale3D (Variables|Default|GetPipe%20Side%202) (Math|Vector|MakeVector (.z _returnvalue_3) (.y _returnvalue_3) (.x _returnvalue_3)))
      (Transformation|SetWorldScale3D (Variables|Default|Get90%20Degree%20Corner) (/ (Variables|Default|GetCorner) 50))
      (Transformation|SetWorldScale3D (Variables|Default|Get45%20Degree%20Corner) (/ (Variables|Default|GetCorner) 50)))
    (:then_1
      ;[1 1 1] Set the position of the box to fit with the corner variable
      (Transformation|SetRelativeLocation (Variables|Default|GetPipe%20Straight) (/ (Variables|Default|GetCorner) 2) false false)
      (Transformation|SetRelativeLocation (Variables|Default|GetPipe%20Side%201) (/ (Variables|Default|GetCorner) 2) false false)
      (Transformation|SetRelativeLocation (Variables|Default|GetPipe%20Side%202) (/ (Variables|Default|GetCorner) 2) false false)
      (Transformation|SetRelativeLocation (Variables|Default|Get90%20Degree%20Corner) (Math|Vector|MakeVector (.x _returnvalue_4) (.y _returnvalue_4) 0.0) false false)
      (Transformation|SetRelativeLocation (Variables|Default|Get45%20Degree%20Corner) (Math|Vector|MakeVector (.x _returnvalue) (.y _returnvalue) 0.0) false false))
    (:then_2
      ;[1 1 1] Set the material of the box
      (Rendering|Material|SetMaterial (Variables|Default|GetPipe%20Straight) 0 (Variables|Default|GetMain%20Color))
      (Rendering|Material|SetMaterial (Variables|Default|GetPipe%20Side%201) 0 (Variables|Default|GetMain%20Color))
      (Rendering|Material|SetMaterial (Variables|Default|GetPipe%20Side%202) 0 (Variables|Default|GetMain%20Color)))
    (:then_3
      (Rendering|SetVisibility (Variables|Default|GetPipe%20Straight) (Utilities|Select :Index (Variables|Default|GetPipeType) :NewEnumerator0 false :NewEnumerator1 false :NewEnumerator2 true :NewEnumerator3 true) false)
      (Rendering|SetVisibility (Variables|Default|GetPipe%20Side%201) (Utilities|Select :Index (Variables|Default|GetPipeType) :NewEnumerator0 false :NewEnumerator1 false :NewEnumerator2 true :NewEnumerator3 true) false)
      (Rendering|SetVisibility (Variables|Default|GetPipe%20Side%202) (Utilities|Select :Index (Variables|Default|GetPipeType) :NewEnumerator0 false :NewEnumerator1 false :NewEnumerator2 true :NewEnumerator3 false) false)
      (Rendering|SetVisibility (Variables|Default|Get45%20Degree%20Corner) (Utilities|Select :Index (Variables|Default|GetPipeType) :NewEnumerator0 false :NewEnumerator1 true :NewEnumerator2 false :NewEnumerator3 false) false)
      (Rendering|SetVisibility (Variables|Default|Get90%20Degree%20Corner) (Utilities|Select :Index (Variables|Default|GetPipeType) :NewEnumerator0 true :NewEnumerator1 false :NewEnumerator2 false :NewEnumerator3 false) false))))