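; BP_DynamicWalls is a level-design blockout actor that generates a wall as a Geometry Script box with a configurable size and material.
; On rebuild it offsets the box by half its X/Y size to pivot from a corner.
; An optional boolean subtracts a second box from a pooled compute mesh, previewed with a brief debug box.
; BakeToStaticMesh copies the result into an assigned static mesh asset.
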(event Custom|Bake%20To%20Static%20Mesh
  (bind _returnvalue (DynamicMeshComponent|GetDynamicMesh (Variables|DynamicMeshActor|GetDynamicMeshComponent)))
  (bind _target_mesh (Variables|Default|GetTarget%20Mesh)
    (:then
      (GeometryScript|StaticMesh|CopyMeshtoStaticMesh :FromDynamicMesh _returnvalue :ToStaticMeshAsset _target_mesh :Debug 0))
    (:else)))

(event Events|EventOnRebuildGeneratedMesh
  (params (TargetMesh :type Dynamic%20Mesh%20Object%20Reference))
  (bind _returnvalue (Transformation|GetActorLocation))
  (bind _boxsize (Variables|Default|GetBoxSize))
  (bind _boolsize (Variables|Default|GetBoolSize))
  (bind _boollocation (Variables|Default|GetBoolLocation))
  (bind _boolsize_2 (Variables|Default|GetBoolSize))
  (bind (_x _y) (Math|Vector|BreakVector _boxsize))
  (bind _returnvalue_2 (Math|Vector|VectorGetAbs _boxsize))
  (bind _returnvalue_3 (Math|Vector|VectorGetAbs _boolsize))
  (bind _returnvalue_4 (+ _boollocation _returnvalue))
  (bind _returnvalue_5 (/ (Math|Vector|MakeVector _x _y 0.0) 2))
  (bind _output_get (Variables|Default|SetDynamic%20Mesh TargetMesh))
  (bind _returnvalue_6 (Class|GeometryScriptLibraryMeshPrimitiveFunctions|AppendBox :TargetMesh _output_get :Transform (Math|Transform|MakeTransform (Math|Vector|MakeVector (.x _returnvalue_5) (.y _returnvalue_5) 0.0) "0, 0, 0" "1.000000,1.000000,1.000000") :DimensionX (.x _returnvalue_2) :DimensionY (.y _returnvalue_2) :DimensionZ (.z _returnvalue_2) :Debug 0))
  ;[1 1 1] Create material
  (GeometryScript|Materials|RemapMaterialIDs _returnvalue_6 0 0 0)
  (Class|DynamicMeshComponent|ConfigureMaterialSet (Variables|DynamicMeshActor|GetDynamicMeshComponent) (Utilities|Array|MakeArray (Variables|Default|GetMaterial)))
  (if (Variables|Default|GetHasBoolean)
    ;[1 1 1] Create and apply boolean mesh
    (bind _returnvalue_7 (Class|DynamicMeshActor|GetComputeMeshPool))
    (bind _returnvalue_8 (Class|DynamicMeshPool|RequestMesh _returnvalue_7))
    (bind _returnvalue_9 (Class|GeometryScriptLibraryMeshPrimitiveFunctions|AppendBox :TargetMesh _returnvalue_8 :Transform (Math|Transform|MakeTransform (Variables|Default|GetBoolLocation) "0, 0, 0" "1.000000,1.000000,1.000000") :DimensionX (.x _returnvalue_3) :DimensionY (.y _returnvalue_3) :DimensionZ (.z _returnvalue_3) :Debug 0))
    (bind _output_get_2 (Variables|Default|SetBoolMesh _returnvalue_9))
    (GeometryScript|Booleans|ApplyMeshBoolean :TargetMesh (Variables|Default|GetDynamic%20Mesh) :ToolMesh _output_get_2 :Operation "Subtract" :Debug 0)
    ;[1 1 1] Preview the bool mesh
    (Rendering|Debug|FlushPersistentDebugLines)
    (Rendering|Debug|DrawDebugBox :Center (Math|Vector|MakeVector (.x _returnvalue_4) (.y _returnvalue_4) (+ (.z _returnvalue_4) (/ (.Z (Math|Vector|BreakVector _boolsize_2)) 2.0))) :Extent (/ _boolsize_2 2) :Duration 1.0 :Thickness 1.0)))

(fn ConstructionScript)