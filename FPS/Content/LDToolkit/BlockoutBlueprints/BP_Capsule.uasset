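; Level-design blockout capsule, built from a Cylinder body with Top and Bottom cap components and resized through a Corner vector.
; The construction script takes diameter from Corner X and total height from Corner Z, shortening the cylinder to fit the caps; Corner Y is ignored.
; Parts are offset so the actor origin sits at a bounding-box corner, and all share the MainColor material.
; The event graph has no active logic.
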(event EventBeginPlay
  (|CallParentFunction) ; This node is disabled and will not be called.\nDrag off pins to build functionality.
)

(event Collision|EventActorBeginOverlap
  (params (OtherActor :type Actor%20Object%20Reference))
  (|CallParentFunction OtherActor) ; This node is disabled and will not be called.\nDrag off pins to build functionality.
)

(event EventTick
  (params (DeltaSeconds :type Float%20%28single-precision%29))
  (|CallParentFunction DeltaSeconds) ; This node is disabled and will not be called.\nDrag off pins to build functionality.
)

(fn ConstructionScript
  (bind _corner (Variables|Default|GetCorner))
  (bind _corner_2 (Variables|Default|GetCorner))
  (bind _corner_3 (Variables|Default|GetCorner))
  (bind _corner_4 (Variables|Default|GetCorner))
  (bind _corner_5 (Variables|Default|GetCorner))
  (bind _corner_6 (Variables|Default|GetCorner))
  (bind _returnvalue (/ (.x _corner_2) 1e+02))
  (bind _returnvalue_2 (/ (.x _corner_6) 2.0))
  (bind _returnvalue_3 (/ (.x _corner_5) 1e+02))
  (bind _returnvalue_4 (/ (.x _corner_4) 1e+02))
  (bind _returnvalue_5 (/ (.x _corner_3) 2.0))
  (bind _returnvalue_6 (/ (.x _corner) 2.0))
  (|CallParentFunction)
  (Transformation|SetRelativeScale3D (Variables|Default|GetCylinder) (Math|Vector|MakeVector _returnvalue _returnvalue (- (/ (.z _corner_2) 1e+02) (/ (.x _corner_2) 1e+02))))
  (Transformation|SetRelativeLocation (Variables|Default|GetCylinder) (Math|Vector|MakeVector _returnvalue_5 _returnvalue_5 (/ (.z _corner_3) 2.0)) false false)
  (Transformation|SetRelativeScale3D (Variables|Default|GetTop) (Math|Vector|MakeVector _returnvalue_4 _returnvalue_4 _returnvalue_4))
  (Transformation|SetRelativeLocation (Variables|Default|GetTop) (Math|Vector|MakeVector _returnvalue_6 _returnvalue_6 (- (.z _corner) (/ (.x _corner) 2.0))) false false)
  (Transformation|SetRelativeScale3D (Variables|Default|GetBottom) (Math|Vector|MakeVector _returnvalue_3 _returnvalue_3 _returnvalue_3))
  (Transformation|SetRelativeLocation (Variables|Default|GetBottom) (Math|Vector|MakeVector _returnvalue_2 _returnvalue_2 (/ (.x _corner_6) 2.0)) false false)
  (Rendering|Material|SetMaterial (Variables|Default|GetTop) 0 (Variables|Default|GetMain%20Color))
  (Rendering|Material|SetMaterial (Variables|Default|GetBottom) 0 (Variables|Default|GetMain%20Color))
  (Rendering|Material|SetMaterial (Variables|Default|GetCylinder) 0 (Variables|Default|GetMain%20Color)))