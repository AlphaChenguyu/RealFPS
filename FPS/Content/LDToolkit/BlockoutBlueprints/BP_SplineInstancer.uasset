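; BP_SplineInstancer is a level-design blockout tool that fills a spline with a chosen static mesh at construction time.
; In deformed mode it chains collidable spline mesh components, one per mesh X length, with tangents clamped to that length.
; Otherwise it adds instanced static mesh instances at intervals of scaled mesh length plus a configurable gap, optionally rotated to follow the spline.
; Segment and instance counts derive from spline length.
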(fn ConstructionScript
  (bind _static_mesh (Variables|Default|GetStatic%20Mesh))
  (bind _meshscale (Variables|Default|GetMeshScale))
  (bind _static_mesh_2 (Variables|Default|GetStatic%20Mesh))
  (bind _meshscale_2 (Variables|Default|GetMeshScale))
  (bind _returnvalue (StaticMesh|GetBoundingBox _static_mesh_2))
  (bind _returnvalue_2 (StaticMesh|GetBoundingBox _static_mesh))
  (if (Variables|Default|GetIsDeformed)
    (Variables|Default|SetX%20Length (.x (+ (Math|Vector|VectorGetAbs (.min _returnvalue_2)) (Math|Vector|VectorGetAbs (.max _returnvalue_2)))))
    (for _index (range 0 (Math|Float|Truncate (/ (Spline|GetSplineLength (Variables|Default|GetSpline)) (Variables|Default|GetX%20Length))))
      (bind _returnvalue_3 (AddComponent|AddSplineMeshComponent false))
      (Collision|SetCollisionEnabled _returnvalue_3 "QueryAndPhysics")
      (SplineMesh|SetForwardAxis _returnvalue_3 "X" true)
      (Components|StaticMesh|SetStaticMesh _returnvalue_3 (Variables|Default|GetStatic%20Mesh))
      (bind (_location _tangent) (CallFunction|GetLocationandTangentAlongSpline (+ 1 _index)))
      (bind (_location_2 _tangent_2) (CallFunction|GetLocationandTangentAlongSpline _index))
      (SplineMesh|SetStartandEnd _returnvalue_3 _location_2 _tangent_2 _location _tangent true :!class /Script/Engine.SplineMeshComponent)
      (SplineMesh|SetEndScale _returnvalue_3 (Math|Vector2D|MakeVector2D _meshscale_2 _meshscale_2) true :!class /Script/Engine.SplineMeshComponent)
      (SplineMesh|SetStartScale _returnvalue_3 (Math|Vector2D|MakeVector2D _meshscale _meshscale) true :!class /Script/Engine.SplineMeshComponent))
    (else
      (Components|StaticMesh|SetStaticMesh (Variables|Default|GetInstancedStaticMesh) (Variables|Default|GetStatic%20Mesh))
      (bind _output_get (Variables|Default|SetX%20Length (* (.x (+ (Math|Vector|VectorGetAbs (.min _returnvalue)) (Math|Vector|VectorGetAbs (.max _returnvalue)))) (Variables|Default|GetMeshScale))))
      (Variables|Default|SetSpaced%20X%20Lnegth (+ _output_get (Variables|Default|GetDistance%20between%20meshes)))
      (for _index_2 (range 0 (Math|Float|Truncate (/ (Spline|GetSplineLength (Variables|Default|GetSpline)) (Variables|Default|GetSpaced%20X%20Lnegth))))
        (Components|InstancedStaticMesh|AddInstance (Variables|Default|GetInstancedStaticMesh) (Math|Transform|MakeTransform (.location (Spline|GetTransformatDistanceAlongSpline (Variables|Default|GetSpline) (* _index_2 (Variables|Default|GetSpaced%20X%20Lnegth)) "Local" false)) (Math|Rotator|SelectRotator (.rotation (Spline|GetTransformatDistanceAlongSpline (Variables|Default|GetSpline) (* _index_2 (Variables|Default|GetSpaced%20X%20Lnegth)) "Local" false)) "0, 0, 0" (Variables|Default|GetRotateMesh)) (* (.scale (Spline|GetTransformatDistanceAlongSpline (Variables|Default|GetSpline) (* _index_2 (Variables|Default|GetSpaced%20X%20Lnegth)) "Local" false)) (Variables|Default|GetMeshScale))) false)))))

(fn GetLocationandTangentAlongSpline
  (params (Index :type Integer))
  (bind _x_length (Variables|Default|GetX%20Length))
  (bind _returnvalue (* Index _x_length))
  (return (Spline|GetLocationatDistanceAlongSpline (Variables|Default|GetSpline) _returnvalue "Local") (Math|Vector|ClampVectorSize (Spline|GetTangentatDistanceAlongSpline (Variables|Default|GetSpline) _returnvalue "Local") 0.0 (Variables|Default|GetX%20Length))))