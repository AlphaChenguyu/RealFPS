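; Blockout chair for level design, built from a seat, a back and four legs.
; The construction script scales and positions each part from a Corner vector and a Thickness value, so the chair fits the box between its origin and that corner.
; The seat sits at mid-height, with legs below and the back rising above along one edge.
; A single MainColor material is applied to every part.
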(fn ConstructionScript
  (bind _corner (Variables|Default|GetCorner))
  (bind _corner_2 (Variables|Default|GetCorner))
  (bind _corner_3 (Variables|Default|GetCorner))
  (bind _thickness (Variables|Default|GetThickness))
  (bind _thickness_2 (Variables|Default|GetThickness))
  (bind _thickness_3 (Variables|Default|GetThickness))
  (bind _thickness_4 (Variables|Default|GetThickness))
  (bind _thickness_5 (Variables|Default|GetThickness))
  (bind _thickness_6 (Variables|Default|GetThickness))
  (bind _thickness_7 (Variables|Default|GetThickness))
  (bind _corner_4 (Variables|Default|GetCorner))
  (bind _thickness_8 (Variables|Default|GetThickness))
  (bind _returnvalue (* _thickness 5e+01))
  (bind _returnvalue_2 (/ _corner_3 100))
  (bind _returnvalue_3 (* _thickness_6 5e+01))
  (bind _returnvalue_4 (* _thickness_7 5e+01))
  (bind _returnvalue_5 (* _thickness_8 5e+01))
  (bind _returnvalue_6 (- _corner_4 (Math|Vector|MakeVector _returnvalue_5 _returnvalue_5 0.0)))
  (|CallParentFunction)
  (Utilities|FlowControl|Sequence
    (:then_0
      (Transformation|SetRelativeScale3D (Variables|Default|GetSeat) (Math|Vector|MakeVector (.x _returnvalue_2) (.y _returnvalue_2) (Variables|Default|GetThickness)))
      (Transformation|SetRelativeScale3D (Variables|Default|GetBack) (Math|Vector|MakeVector (Variables|Default|GetThickness) (/ (.y _corner) 1e+02) (/ (- (.z _corner) (* (Variables|Default|GetThickness) 1e+02)) 2e+02)))
      (Transformation|SetRelativeScale3D (Variables|Default|GetLeg1) (Math|Vector|MakeVector _thickness_4 _thickness_4 (/ (- (.z (Variables|Default|GetCorner)) (* (Variables|Default|GetThickness) 1e+02)) 2e+02)))
      (Transformation|SetRelativeScale3D (Variables|Default|GetLeg2) (Math|Vector|MakeVector _thickness_5 _thickness_5 (/ (- (.z (Variables|Default|GetCorner)) (* (Variables|Default|GetThickness) 1e+02)) 2e+02)))
      (Transformation|SetRelativeScale3D (Variables|Default|GetLeg3) (Math|Vector|MakeVector _thickness_3 _thickness_3 (/ (- (.z (Variables|Default|GetCorner)) (* (Variables|Default|GetThickness) 1e+02)) 2e+02)))
      (Transformation|SetRelativeScale3D (Variables|Default|GetLeg4) (Math|Vector|MakeVector _thickness_2 _thickness_2 (/ (- (.z (Variables|Default|GetCorner)) (* (Variables|Default|GetThickness) 1e+02)) 2e+02))))
    (:then_1
      (Transformation|SetRelativeLocation (Variables|Default|GetLeg1) (Math|Vector|MakeVector _returnvalue _returnvalue (/ (- (.z (Variables|Default|GetCorner)) (* (Variables|Default|GetThickness) 1e+02)) 4.0)) false false)
      (Transformation|SetRelativeLocation (Variables|Default|GetLeg2) (Math|Vector|MakeVector (- (.x (Variables|Default|GetCorner)) _returnvalue_3) _returnvalue_3 (/ (- (.z (Variables|Default|GetCorner)) (* (Variables|Default|GetThickness) 1e+02)) 4.0)) false false)
      (Transformation|SetRelativeLocation (Variables|Default|GetLeg3) (Math|Vector|MakeVector (.x _returnvalue_6) (.y _returnvalue_6) (/ (- (.z (Variables|Default|GetCorner)) (* (Variables|Default|GetThickness) 1e+02)) 4.0)) false false)
      (Transformation|SetRelativeLocation (Variables|Default|GetLeg4) (Math|Vector|MakeVector _returnvalue_4 (- (.y (Variables|Default|GetCorner)) _returnvalue_4) (/ (- (.z (Variables|Default|GetCorner)) (* (Variables|Default|GetThickness) 1e+02)) 4.0)) false false)
      (Transformation|SetRelativeLocation (Variables|Default|GetSeat) (/ (Variables|Default|GetCorner) 2) false false)
      (Transformation|SetRelativeLocation (Variables|Default|GetBack) (Math|Vector|MakeVector (* (Variables|Default|GetThickness) 5e+01) (/ (.y _corner_2) 2.0) (+ (/ (.z _corner_2) 2.0) (/ (.z _corner_2) 4.0) (* (Variables|Default|GetThickness) 25.0))) false false))
    (:then_2
      (Rendering|Material|SetMaterial (Variables|Default|GetBack) 0 (Variables|Default|GetMain%20Color))
      (Rendering|Material|SetMaterial (Variables|Default|GetLeg4) 0 (Variables|Default|GetMain%20Color))
      (Rendering|Material|SetMaterial (Variables|Default|GetLeg3) 0 (Variables|Default|GetMain%20Color))
      (Rendering|Material|SetMaterial (Variables|Default|GetLeg2) 0 (Variables|Default|GetMain%20Color))
      (Rendering|Material|SetMaterial (Variables|Default|GetLeg1) 0 (Variables|Default|GetMain%20Color))
      (Rendering|Material|SetMaterial (Variables|Default|GetSeat) 0 (Variables|Default|GetMain%20Color)))))