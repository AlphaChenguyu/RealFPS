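; BP_PipeStraight is a level design blockout Blueprint for a straight pipe piece sized by a Corner variable.
; The construction script sets the Pipe component's world scale to Corner divided by 50 and its relative location to half of Corner, fitting it between the actor origin and that corner.
; It also applies MainColor as the material; the event graph holds only disabled stub events.
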(event EventBeginPlay
  (|CallParentFunction) ; This node is disabled and will not be called.\nDrag off pins to build functionality.
)

(event Collision|EventActorBeginOverlap
  (params (OtherActor :type Actor%20Object%20Reference))
  (|CallParentFunction OtherActor) ; This node is disabled and will not be called.\nDrag off pins to build functionality.
)

(event EventTick
  (params (DeltaSeconds :type Float%20%28single-precision%29))
  (|CallParentFunction DeltaSeconds) ; This node is disabled and will not be called.\nDrag off pins to build functionality.
)

(fn ConstructionScript
  (|CallParentFunction)
  (Utilities|FlowControl|Sequence
    (:then_0
      ;[1 1 1] Set the scale of the box based on the corner variable
      (Transformation|SetWorldScale3D (Variables|Default|GetPipe) (/ (Variables|Default|GetCorner) 50)))
    (:then_1
      ;[1 1 1] Set the position of the box to fit with the corner variable
      (Transformation|SetRelativeLocation (Variables|Default|GetPipe) (/ (Variables|Default|GetCorner) 2) false false))
    (:then_2
      ;[1 1 1] Set the material of the box
      (Rendering|Material|SetMaterial (Variables|Default|GetPipe) 0 (Variables|Default|GetMain%20Color)))))