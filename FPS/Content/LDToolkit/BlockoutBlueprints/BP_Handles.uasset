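; Level-design blockout Blueprint that builds a parametric U-shaped handle from three cylinders and two corner meshes.
; Its construction script, after calling the parent's, scales and positions the parts from the Corner point's X and Z and a Thickness value.
; A vertical bar joins two horizontal bars through the corner pieces, with offsets keeping the shape inside the Corner bounds.
; All five parts share the MainColor material.
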(fn ConstructionScript
  (bind _thickness (Variables|Default|GetThickness))
  (bind _thickness_2 (Variables|Default|GetThickness))
  (bind _thickness_3 (Variables|Default|GetThickness))
  (bind _corner (Variables|Default|GetCorner))
  (bind _corner_2 (Variables|Default|GetCorner))
  (bind _corner_3 (Variables|Default|GetCorner))
  (bind _thickness_4 (Variables|Default|GetThickness))
  (bind _thickness_5 (Variables|Default|GetThickness))
  (bind _thickness_6 (Variables|Default|GetThickness))
  (bind _thickness_7 (Variables|Default|GetThickness))
  (bind _returnvalue (* _thickness 2.0))
  (bind _returnvalue_2 (* _thickness_7 2.0))
  (bind _returnvalue_3 (* _thickness_4 5e+01))
  (bind _returnvalue_4 (* _thickness_5 5e+01))
  (|CallParentFunction)
  (Utilities|FlowControl|Sequence
    (:then_0
      (Transformation|SetRelativeScale3D (Variables|Default|GetStaticMesh) (Math|Vector|MakeVector _returnvalue_2 _returnvalue_2 _returnvalue_2))
      (Transformation|SetRelativeScale3D (Variables|Default|GetStaticMesh1) (Math|Vector|MakeVector _returnvalue _returnvalue _returnvalue))
      (Transformation|SetRelativeScale3D (Variables|Default|GetCylinder2) (Math|Vector|MakeVector _thickness_2 _thickness_2 (- (/ (.z (Variables|Default|GetCorner)) 1e+02) (* (Variables|Default|GetThickness) 2.0))))
      (Transformation|SetRelativeScale3D (Variables|Default|GetCylinder1) (Math|Vector|MakeVector _thickness_3 _thickness_3 (- (/ (.x (Variables|Default|GetCorner)) 1e+02) (Variables|Default|GetThickness))))
      (Transformation|SetRelativeScale3D (Variables|Default|GetCylinder) (Math|Vector|MakeVector _thickness_6 _thickness_6 (- (/ (.x (Variables|Default|GetCorner)) 1e+02) (Variables|Default|GetThickness)))))
    (:then_1
      (Transformation|SetRelativeLocation (Variables|Default|GetStaticMesh) (Math|Vector|MakeVector (- (.x _corner) _returnvalue_4) 0.0 (- (.z _corner) _returnvalue_4)) false false)
      (Transformation|SetRelativeLocation (Variables|Default|GetStaticMesh1) (Math|Vector|MakeVector (- (.x (Variables|Default|GetCorner)) _returnvalue_3) 0.0 _returnvalue_3) false false)
      (Transformation|SetRelativeLocation (Variables|Default|GetCylinder2) (Math|Vector|MakeVector (- (.x _corner_3) (* (Variables|Default|GetThickness) 5e+01)) 0.0 (/ (.z _corner_3) 2.0)) false false)
      (Transformation|SetRelativeLocation (Variables|Default|GetCylinder1) (Math|Vector|MakeVector (/ (- (.x (Variables|Default|GetCorner)) (* (Variables|Default|GetThickness) 1e+02)) 2.0) 0.0 (* (Variables|Default|GetThickness) 5e+01)) false false)
      (Transformation|SetRelativeLocation (Variables|Default|GetCylinder) (Math|Vector|MakeVector (/ (- (.x _corner_2) (* (Variables|Default|GetThickness) 1e+02)) 2.0) 0.0 (- (.z _corner_2) (* (Variables|Default|GetThickness) 5e+01))) false false))
    (:then_2
      (Rendering|Material|SetMaterial (Variables|Default|GetStaticMesh1) 0 (Variables|Default|GetMain%20Color))
      (Rendering|Material|SetMaterial (Variables|Default|GetStaticMesh) 0 (Variables|Default|GetMain%20Color))
      (Rendering|Material|SetMaterial (Variables|Default|GetCylinder2) 0 (Variables|Default|GetMain%20Color))
      (Rendering|Material|SetMaterial (Variables|Default|GetCylinder1) 0 (Variables|Default|GetMain%20Color))
      (Rendering|Material|SetMaterial (Variables|Default|GetCylinder) 0 (Variables|Default|GetMain%20Color)))))