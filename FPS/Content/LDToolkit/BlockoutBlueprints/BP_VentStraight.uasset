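; Blockout level-design actor that builds a straight vent section from four cube meshes forming a hollow rectangular duct open along X.
; The construction script sizes and places two side walls and a top and bottom panel from CornerPosition and OuterThickness, keeping them within the box from the actor origin to that corner.
; It then applies MainColor as the material on all four cubes; the event graph has no active logic.
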(event EventBeginPlay
  (|CallParentFunction) ; This node is disabled and will not be called.\nDrag off pins to build functionality.
)

(event Collision|EventActorBeginOverlap
  (params (OtherActor :type Actor%20Object%20Reference))
  (|CallParentFunction OtherActor) ; This node is disabled and will not be called.\nDrag off pins to build functionality.
)

(event EventTick
  (params (DeltaSeconds :type Float%20%28single-precision%29))
  (|CallParentFunction DeltaSeconds) ; This node is disabled and will not be called.\nDrag off pins to build functionality.
)

(fn ConstructionScript
  (|CallParentFunction)
  (Utilities|FlowControl|Sequence
    (:then_0
      ;[1 1 1] Scale the frames based on the corner
      (CallFunction|VerticalScaling (Variables|Default|GetCube))
      (CallFunction|VerticalScaling (Variables|Default|GetCube1))
      (CallFunction|HorizontalScaling (Variables|Default|GetCube2))
      (CallFunction|HorizontalScaling (Variables|Default|GetCube3)))
    (:then_1
      ;[1 1 1] Move the frames based on the corner
      (CallFunction|VerticalPositioning (Variables|Default|GetCube) 0.0 (- (.y (Variables|Default|GetCornerPosition)) (* (Variables|Default|GetOuter%20Thickness) 5e+01)))
      (CallFunction|VerticalPositioning (Variables|Default|GetCube1) 5.0 (* (Variables|Default|GetOuter%20Thickness) 5e+01))
      (CallFunction|HorizontalPositioning (Variables|Default|GetCube2) 0.0 (- (.z (Variables|Default|GetCornerPosition)) (* (Variables|Default|GetOuter%20Thickness) 5e+01)))
      (CallFunction|HorizontalPositioning (Variables|Default|GetCube3) 0.0 (* (Variables|Default|GetOuter%20Thickness) 5e+01)))
    (:then_3
      ;[1 1 1] Set material of cubes
      (for _index (range 0 3)
        (Rendering|Material|SetMaterial (Utilities|Select :Index _index :Option%200 (Variables|Default|GetCube) :Option%201 (Variables|Default|GetCube1) :Option%202 (Variables|Default|GetCube2) :Option%203 (Variables|Default|GetCube3)) 0 (Variables|Default|GetMain%20Color))))))

(fn VerticalScaling
  (params (self2 :type Scene%20Component%20Object%20Reference))
  (bind _cornerposition (Variables|Default|GetCornerPosition))
  (Transformation|SetRelativeScale3D self2 (Math|Vector|MakeVector (/ (.x _cornerposition) 1e+02) (Variables|Default|GetOuter%20Thickness) (/ (.z _cornerposition) 1e+02))))

(fn HorizontalScaling
  (params (self2 :type Scene%20Component%20Object%20Reference))
  (bind _cornerposition (Variables|Default|GetCornerPosition))
  (Transformation|SetRelativeScale3D self2 (Math|Vector|MakeVector (/ (.x _cornerposition) 1e+02) (/ (.y _cornerposition) 1e+02) (Variables|Default|GetOuter%20Thickness))))

(fn VerticalPositioning
  (params (self2 :type Scene%20Component%20Object%20Reference) (New%20Location%20X :type Float%20%28double-precision%29) (New%20Location%20Y :type Float%20%28double-precision%29))
  (bind _cornerposition (Variables|Default|GetCornerPosition))
  (Transformation|SetRelativeLocation self2 (Math|Vector|MakeVector (/ (.x _cornerposition) 2.0) New%20Location%20Y (/ (.z _cornerposition) 2.0)) false false))

(fn HorizontalPositioning
  (params (self2 :type Scene%20Component%20Object%20Reference) (New%20Location%20Y :type Float%20%28double-precision%29) (New%20Location%20Z :type Float%20%28double-precision%29))
  (bind _cornerposition (Variables|Default|GetCornerPosition))
  (Transformation|SetRelativeLocation self2 (Math|Vector|MakeVector (/ (.x _cornerposition) 2.0) (/ (.y _cornerposition) 2.0) New%20Location%20Z) false false))