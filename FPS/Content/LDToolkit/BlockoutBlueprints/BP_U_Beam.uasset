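; BP_U_Beam is a blockout Blueprint that builds a resizable U-shaped beam from three mesh pieces.
; Its construction script scales and positions the top, bottom and center pieces from a Corner vector, with separate thicknesses for outer and center beams.
; Offsets keep the pieces inside the box from origin to Corner, assuming 100-unit centered meshes.
; All pieces share the MainColor material, and the event graph has no active logic.
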(event EventBeginPlay
  (|CallParentFunction) ; This node is disabled and will not be called.\nDrag off pins to build functionality.
)

(event Collision|EventActorBeginOverlap
  (params (OtherActor :type Actor%20Object%20Reference))
  (|CallParentFunction OtherActor) ; This node is disabled and will not be called.\nDrag off pins to build functionality.
)

(event EventTick
  (params (DeltaSeconds :type Float%20%28single-precision%29))
  (|CallParentFunction DeltaSeconds) ; This node is disabled and will not be called.\nDrag off pins to build functionality.
)

(fn ConstructionScript
  (bind _corner (Variables|Default|GetCorner))
  (bind _corner_2 (Variables|Default|GetCorner))
  (bind _corner_3 (Variables|Default|GetCorner))
  (bind _corner_4 (Variables|Default|GetCorner))
  (bind _corner_5 (Variables|Default|GetCorner))
  (bind _corner_6 (Variables|Default|GetCorner))
  (|CallParentFunction)
  (Rendering|Material|SetMaterial (Variables|Default|GetTopPiece) 0 (Variables|Default|GetMain%20Color))
  (Rendering|Material|SetMaterial (Variables|Default|GetBottomPiece) 0 (Variables|Default|GetMain%20Color))
  (Rendering|Material|SetMaterial (Variables|Default|GetCenterPiece) 0 (Variables|Default|GetMain%20Color))
  ;[1 1 1] Set Scale and Location of Top Piece
  (Transformation|SetRelativeScale3D (Variables|Default|GetTopPiece) (Math|Vector|MakeVector (Variables|Default|GetOuter%20Beam%20Thickness) (/ (.y _corner_3) 1e+02) (/ (.z _corner_3) 1e+02)))
  (Transformation|SetRelativeLocation (Variables|Default|GetTopPiece) (Math|Vector|MakeVector (- (.x _corner_4) (* (Variables|Default|GetOuter%20Beam%20Thickness) 5e+01)) (/ (.y _corner_4) 2.0) (/ (.z _corner_4) 2.0)) false false)
  ;[1 1 1] Set Scale and Location of Bottom Piece
  (Transformation|SetRelativeScale3D (Variables|Default|GetBottomPiece) (Math|Vector|MakeVector (Variables|Default|GetOuter%20Beam%20Thickness) (/ (.y _corner) 1e+02) (/ (.z _corner) 1e+02)))
  (Transformation|SetRelativeLocation (Variables|Default|GetBottomPiece) (Math|Vector|MakeVector (* (Variables|Default|GetOuter%20Beam%20Thickness) 5e+01) (/ (.y _corner_2) 2.0) (/ (.z _corner_2) 2.0)) false false)
  (Transformation|SetRelativeScale3D (Variables|Default|GetCenterPiece) (Math|Vector|MakeVector (/ (.x _corner_5) 1e+02) (Variables|Default|GetCenter%20Beam%20Thickness) (/ (.z _corner_5) 1e+02)))
  (Transformation|SetRelativeLocation (Variables|Default|GetCenterPiece) (Math|Vector|MakeVector (/ (.x _corner_6) 2.0) (* (Variables|Default|GetCenter%20Beam%20Thickness) 5e+01) (/ (.z _corner_6) 2.0)) false false))