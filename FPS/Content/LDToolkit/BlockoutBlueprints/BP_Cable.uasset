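; BP_Cable is a level blockout actor that builds a cable along an editable spline, with configurable width and material.
; Its construction script places an instanced corner mesh at every spline point and an instanced straight mesh between each consecutive pair.
; Straights sit at segment midpoints, aimed with look-at rotation and stretched to the point distance, so the cable ignores spline curvature.
; It has no active runtime logic.
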(event EventBeginPlay
  (|CallParentFunction) ; This node is disabled and will not be called.\nDrag off pins to build functionality.
)

(event Collision|EventActorBeginOverlap
  (params (OtherActor :type Actor%20Object%20Reference))
  (|CallParentFunction OtherActor) ; This node is disabled and will not be called.\nDrag off pins to build functionality.
)

(event EventTick
  (params (DeltaSeconds :type Float%20%28single-precision%29))
  (|CallParentFunction DeltaSeconds) ; This node is disabled and will not be called.\nDrag off pins to build functionality.
)

(fn ConstructionScript
  (bind _cablewidth (Variables|Default|GetCableWidth))
  (|CallParentFunction)
  (Rendering|Material|SetMaterial (Variables|Default|GetCableCorners) 0 (Variables|Default|GetMain%20Color))
  (Rendering|Material|SetMaterial (Variables|Default|GetCableStraights) 0 (Variables|Default|GetMain%20Color))
  (for _index (range 0 (- (Spline|GetNumberOfSplinePoints (Variables|Default|GetSpline)) 1))
    (Components|InstancedStaticMesh|AddInstance (Variables|Default|GetCableCorners) (Math|Transform|MakeTransform (.position (Spline|GetSplinePointAt (Variables|Default|GetSpline) _index "Local")) "0, 0, 0" (Math|Conversions|ToVector(Float) (/ (Variables|Default|GetCableWidth) 1.65))) false)
    (if (> _index 0)
      (Components|InstancedStaticMesh|AddInstance (Variables|Default|GetCableStraights) (Math|Transform|MakeTransform (+ (.position (Spline|GetSplinePointAt (Variables|Default|GetSpline) _index "Local")) (/ (- (.position (Spline|GetSplinePointAt (Variables|Default|GetSpline) (- _index 1) "Local")) (.position (Spline|GetSplinePointAt (Variables|Default|GetSpline) _index "Local"))) 2)) (Math|Rotator|FindLookatRotation (.position (Spline|GetSplinePointAt (Variables|Default|GetSpline) _index "Local")) (.position (Spline|GetSplinePointAt (Variables|Default|GetSpline) (- _index 1) "Local"))) (Math|Vector|MakeVector (/ (Math|Vector|VectorLength (- (.position (Spline|GetSplinePointAt (Variables|Default|GetSpline) _index "Local")) (.position (Spline|GetSplinePointAt (Variables|Default|GetSpline) (- _index 1) "Local")))) 2e+02) _cablewidth _cablewidth)) false))))