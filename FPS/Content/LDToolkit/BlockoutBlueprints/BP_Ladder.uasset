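; BP_Ladder is a level-design blockout ladder built procedurally in the construction script, with no active gameplay logic.
; Two cube rails are scaled and placed from the Corner vector and Thickness, so Corner X sets the width and Z the height.
; An instanced static mesh fills the gap between the rails with rungs spaced by RungDistance, all sharing the MainColor material.
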(event EventBeginPlay
  (|CallParentFunction) ; This node is disabled and will not be called.\nDrag off pins to build functionality.
)

(event Collision|EventActorBeginOverlap
  (params (OtherActor :type Actor%20Object%20Reference))
  (|CallParentFunction OtherActor) ; This node is disabled and will not be called.\nDrag off pins to build functionality.
)

(event EventTick
  (params (DeltaSeconds :type Float%20%28single-precision%29))
  (|CallParentFunction DeltaSeconds) ; This node is disabled and will not be called.\nDrag off pins to build functionality.
)

(fn ConstructionScript
  (bind _thickness (Variables|Default|GetThickness))
  (bind _thickness_2 (Variables|Default|GetThickness))
  (bind _thickness_3 (Variables|Default|GetThickness))
  (bind _thickness_4 (Variables|Default|GetThickness))
  (bind _corner (Variables|Default|GetCorner))
  (bind _thickness_5 (Variables|Default|GetThickness))
  (bind _corner_2 (Variables|Default|GetCorner))
  (bind _returnvalue (* _thickness 5e+01))
  (bind _returnvalue_2 (* _thickness_4 5e+01))
  (|CallParentFunction)
  (Rendering|Material|SetMaterial (Variables|Default|GetCube) 0 (Variables|Default|GetMain%20Color))
  (Rendering|Material|SetMaterial (Variables|Default|GetCube1) 0 (Variables|Default|GetMain%20Color))
  (Transformation|SetRelativeScale3D (Variables|Default|GetCube1) (Math|Vector|MakeVector _thickness_2 _thickness_2 (/ (.z (Variables|Default|GetCorner)) 1e+02)))
  (Transformation|SetRelativeLocation (Variables|Default|GetCube1) (Math|Vector|MakeVector (- (.x _corner_2) _returnvalue_2) _returnvalue_2 (/ (.z _corner_2) 2.0)) false false)
  (Transformation|SetRelativeScale3D (Variables|Default|GetCube) (Math|Vector|MakeVector _thickness_3 _thickness_3 (/ (.z (Variables|Default|GetCorner)) 1e+02)))
  (Transformation|SetRelativeLocation (Variables|Default|GetCube) (Math|Vector|MakeVector _returnvalue _returnvalue (/ (.z (Variables|Default|GetCorner)) 2.0)) false false)
  (Components|StaticMesh|SetStaticMesh (Variables|Default|GetInstancedStaticMesh) "/Engine/BasicShapes/Cube.Cube")
  (Rendering|Material|SetMaterial (Variables|Default|GetInstancedStaticMesh) 0 (Variables|Default|GetMain%20Color))
  (for _index (range 1 (- (Math|Float|Floor (/ (.z (Variables|Default|GetCorner)) (Variables|Default|GetRung%20Distance))) 1))
    (Components|InstancedStaticMesh|AddInstance (Variables|Default|GetInstancedStaticMesh) (Math|Transform|MakeTransform (Math|Vector|MakeVector (/ (.x _corner) 2.0) (* (Variables|Default|GetThickness) 5e+01) (+ (* _index (Variables|Default|GetRung%20Distance)) (* (Variables|Default|GetThickness) 5e+01))) "0, 0, 0" (Math|Vector|MakeVector (- (/ (.x _corner) 1e+02) (* (Variables|Default|GetThickness) 2.0)) _thickness_5 _thickness_5)) false)))