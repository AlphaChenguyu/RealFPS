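; BP_Table is a parametric blockout table for level design, built from a top and four legs.
; The construction script sizes and places the parts from a Corner vector, with thickness values for top and legs, scaling on the assumption of 100-unit meshes.
; Legs sit inset at the footprint's corners and reach from the origin plane to the underside of the top.
; One MainColor material is applied to all five parts.
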(fn ConstructionScript
  (bind _corner (Variables|Default|GetCorner))
  (bind _corner_2 (Variables|Default|GetCorner))
  (bind _leg_thickness (Variables|Default|GetLeg%20Thickness))
  (bind _leg_thickness_2 (Variables|Default|GetLeg%20Thickness))
  (bind _leg_thickness_3 (Variables|Default|GetLeg%20Thickness))
  (bind _corner_3 (Variables|Default|GetCorner))
  (bind _leg_thickness_4 (Variables|Default|GetLeg%20Thickness))
  (bind _leg_thickness_5 (Variables|Default|GetLeg%20Thickness))
  (bind _corner_4 (Variables|Default|GetCorner))
  (bind _leg_thickness_6 (Variables|Default|GetLeg%20Thickness))
  (bind _leg_thickness_7 (Variables|Default|GetLeg%20Thickness))
  (bind _corner_5 (Variables|Default|GetCorner))
  (bind _leg_thickness_8 (Variables|Default|GetLeg%20Thickness))
  (bind _returnvalue (* _leg_thickness_2 5e+01))
  (bind _returnvalue_2 (* _leg_thickness_4 5e+01))
  (bind _returnvalue_3 (* _leg_thickness_6 5e+01))
  (bind _returnvalue_4 (* _leg_thickness_8 5e+01))
  (|CallParentFunction)
  (Utilities|FlowControl|Sequence
    (:then_0
      (Transformation|SetRelativeScale3D (Variables|Default|GetTop) (Math|Vector|MakeVector (/ (.x _corner_2) 1e+02) (/ (.y _corner_2) 1e+02) (Variables|Default|GetTop%20Thickness)))
      (Transformation|SetRelativeLocation (Variables|Default|GetTop) (Math|Vector|MakeVector (/ (.x _corner) 2.0) (/ (.y _corner) 2.0) (- (.z _corner) (* (Variables|Default|GetTop%20Thickness) 5e+01))) false false)
      (Transformation|SetRelativeScale3D (Variables|Default|GetLeg1) (Math|Vector|MakeVector _leg_thickness_3 _leg_thickness_3 (- (/ (.z (Variables|Default|GetCorner)) 1e+02) (Variables|Default|GetTop%20Thickness))))
      (Transformation|SetRelativeLocation (Variables|Default|GetLeg1) (Math|Vector|MakeVector (- (.x _corner_3) _returnvalue_2) (- (.y _corner_3) _returnvalue_2) (- (/ (.z _corner_3) 2.0) (* (Variables|Default|GetTop%20Thickness) 5e+01))) false false)
      (Transformation|SetRelativeScale3D (Variables|Default|GetLeg2) (Math|Vector|MakeVector _leg_thickness_5 _leg_thickness_5 (- (/ (.z (Variables|Default|GetCorner)) 1e+02) (Variables|Default|GetTop%20Thickness))))
      (Transformation|SetRelativeLocation (Variables|Default|GetLeg2) (Math|Vector|MakeVector (- (.x _corner_5) _returnvalue_4) _returnvalue_4 (- (/ (.z _corner_5) 2.0) (* (Variables|Default|GetTop%20Thickness) 5e+01))) false false)
      (Transformation|SetRelativeScale3D (Variables|Default|GetLeg3) (Math|Vector|MakeVector _leg_thickness_7 _leg_thickness_7 (- (/ (.z (Variables|Default|GetCorner)) 1e+02) (Variables|Default|GetTop%20Thickness))))
      (Transformation|SetRelativeLocation (Variables|Default|GetLeg3) (Math|Vector|MakeVector _returnvalue _returnvalue (- (/ (.z (Variables|Default|GetCorner)) 2.0) (* (Variables|Default|GetTop%20Thickness) 5e+01))) false false)
      (Transformation|SetRelativeScale3D (Variables|Default|GetLeg4) (Math|Vector|MakeVector _leg_thickness _leg_thickness (- (/ (.z (Variables|Default|GetCorner)) 1e+02) (Variables|Default|GetTop%20Thickness))))
      (Transformation|SetRelativeLocation (Variables|Default|GetLeg4) (Math|Vector|MakeVector _returnvalue_3 (- (.y _corner_4) _returnvalue_3) (- (/ (.z _corner_4) 2.0) (* (Variables|Default|GetTop%20Thickness) 5e+01))) false false))
    (:then_1
      (Rendering|Material|SetMaterial (Variables|Default|GetLeg4) 0 (Variables|Default|GetMain%20Color))
      (Rendering|Material|SetMaterial (Variables|Default|GetLeg3) 0 (Variables|Default|GetMain%20Color))
      (Rendering|Material|SetMaterial (Variables|Default|GetLeg2) 0 (Variables|Default|GetMain%20Color))
      (Rendering|Material|SetMaterial (Variables|Default|GetLeg1) 0 (Variables|Default|GetMain%20Color))
      (Rendering|Material|SetMaterial (Variables|Default|GetTop) 0 (Variables|Default|GetMain%20Color)))))