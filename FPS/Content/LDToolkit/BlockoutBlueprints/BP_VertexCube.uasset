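; BP_VertexCube is a level-design blockout box whose procedural mesh is reshaped through its vertices and six face centers.
; The construction script seeds a box only when Vertices is empty, so stored edits persist across reconstructions.
; A face center that differs from its tracked copy offsets that face's vertices, including coincident corner duplicates.
; It then recomputes centers from opposite corners, rebuilds the mesh with collision and material, and saves the tracked centers.
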(event EventBeginPlay)

(event Collision|EventActorBeginOverlap
  (params (OtherActor :type Actor%20Object%20Reference)))

(event EventTick
  (params (DeltaSeconds :type Float%20%28single-precision%29)))

(fn ConstructionScript
  (bind (_vertices _triangles _normals _uvs _tangents) (Class|KismetProceduralMeshLibrary|GenerateBoxMesh "50.000000,50.000000,50.000000"))
  (if (Utilities|Array|IsEmpty (Variables|Backend|GetVertices))
    (Variables|Backend|SetVertices _vertices)
    (Variables|Backend|SetTriangles _triangles)
    (Variables|Backend|SetNormals _normals)
    (Variables|Backend|SetUV _uvs)
    (Variables|Backend|SetTangents _tangents)
    (for (_array_element _array_index) (Variables|Backend|GetVertices)
      (Utilities|Array|SetArrayElem (Variables|Backend|GetVertices) _array_index (+ _array_element "50.000000,50.000000,50.000000"))
      (Utilities|FlowControl|Sequence
        (:then_0
          (Utilities|FlowControl|Sequence
            (:then_0
              (if (Class|KismetMathLibrary|NotEqualExactlyVectorVector (Variables|Backend|GetCenterTop) (Variables|Backend|GetCenterTrackTop))
                (CallFunction|UpdateVertexPostionThroughCenter (Variables|Backend|GetCenterTop) (Variables|Backend|GetCenterTrackTop) (Utilities|Array|MakeArray 3 6 17 2 13 18 1 9 14 0 5 10)))
              (if (Class|KismetMathLibrary|NotEqualExactlyVectorVector (Variables|Backend|GetCenterLeft) (Variables|Backend|GetCenterTrackLeft))
                (CallFunction|UpdateVertexPostionThroughCenter (Variables|Backend|GetCenterLeft) (Variables|Backend|GetCenterTrackLeft) (Utilities|Array|MakeArray 3 6 17 2 13 18 7 16 20 12 19 21)))
              (if (Class|KismetMathLibrary|NotEqualExactlyVectorVector (Variables|Backend|GetCenterRight) (Variables|Backend|GetCenterTrackRight))
                (CallFunction|UpdateVertexPostionThroughCenter (Variables|Backend|GetCenterRight) (Variables|Backend|GetCenterTrackRight) (Utilities|Array|MakeArray 0 5 10 1 9 14 4 11 23 8 15 22)))
              (if (Class|KismetMathLibrary|NotEqualExactlyVectorVector (Variables|Backend|GetCenterFront) (Variables|Backend|GetCenterTrackFront))
                (CallFunction|UpdateVertexPostionThroughCenter (Variables|Backend|GetCenterFront) (Variables|Backend|GetCenterTrackFront) (Utilities|Array|MakeArray 3 6 17 0 5 10 4 11 23 7 16 20)))
              (if (Class|KismetMathLibrary|NotEqualExactlyVectorVector (Variables|Backend|GetCenterBack) (Variables|Backend|GetCenterTrackBack))
                (CallFunction|UpdateVertexPostionThroughCenter (Variables|Backend|GetCenterBack) (Variables|Backend|GetCenterTrackBack) (Utilities|Array|MakeArray 2 13 18 1 9 14 8 15 22 12 19 21)))
              (if (Class|KismetMathLibrary|NotEqualExactlyVectorVector (Variables|Backend|GetCenterBottom) (Variables|Backend|GetCenterTrackBottom))
                (CallFunction|UpdateVertexPostionThroughCenter (Variables|Backend|GetCenterBottom) (Variables|Backend|GetCenterTrackBottom) (Utilities|Array|MakeArray 7 16 20 4 11 23 8 15 22 12 19 21))))))
        (:then_1
          (bind _caluclated_centerposition (CallFunction|UpdateCenterPosition 0 2))
          (Variables|Backend|SetCenterTop _caluclated_centerposition)
          (bind _caluclated_centerposition_2 (CallFunction|UpdateCenterPosition 2 7))
          (Variables|Backend|SetCenterLeft _caluclated_centerposition_2)
          (bind _caluclated_centerposition_3 (CallFunction|UpdateCenterPosition 0 8))
          (Variables|Backend|SetCenterRight _caluclated_centerposition_3)
          (bind _caluclated_centerposition_4 (CallFunction|UpdateCenterPosition 7))
          (Variables|Backend|SetCenterFront _caluclated_centerposition_4)
          (bind _caluclated_centerposition_5 (CallFunction|UpdateCenterPosition 2 8))
          (Variables|Backend|SetCenterBack _caluclated_centerposition_5)
          (bind _caluclated_centerposition_6 (CallFunction|UpdateCenterPosition 7 8))
          (Variables|Backend|SetCenterBottom _caluclated_centerposition_6))
        (:then_2
          (Class|ProceduralMeshComponent|CreateMeshSectionLinearColor (Variables|Default|GetProceduralMesh) 0 (Variables|Backend|GetVertices) (Variables|Backend|GetTriangles) (Variables|Backend|GetNormals) (Variables|Backend|GetUV) 0 0 0 0 (Variables|Backend|GetTangents) true false)
          (Rendering|Material|SetMaterial (Variables|Default|GetProceduralMesh) 0 (Variables|Default|GetMaterial))
          (Variables|Backend|SetCenterTrackTop (Variables|Backend|GetCenterTop))
          (Variables|Backend|SetCenterTrackLeft (Variables|Backend|GetCenterLeft))
          (Variables|Backend|SetCenterTrackRight (Variables|Backend|GetCenterRight))
          (Variables|Backend|SetCenterTrackFront (Variables|Backend|GetCenterFront))
          (Variables|Backend|SetCenterTrackBack (Variables|Backend|GetCenterBack))
          (Variables|Backend|SetCenterTrackBottom (Variables|Backend|GetCenterBottom)))))
    (else
      (Utilities|FlowControl|Sequence
        (:then_0
          (Utilities|FlowControl|Sequence
            (:then_0
              (if (Class|KismetMathLibrary|NotEqualExactlyVectorVector (Variables|Backend|GetCenterTop) (Variables|Backend|GetCenterTrackTop))
                (CallFunction|UpdateVertexPostionThroughCenter (Variables|Backend|GetCenterTop) (Variables|Backend|GetCenterTrackTop) (Utilities|Array|MakeArray 3 6 17 2 13 18 1 9 14 0 5 10)))
              (if (Class|KismetMathLibrary|NotEqualExactlyVectorVector (Variables|Backend|GetCenterLeft) (Variables|Backend|GetCenterTrackLeft))
                (CallFunction|UpdateVertexPostionThroughCenter (Variables|Backend|GetCenterLeft) (Variables|Backend|GetCenterTrackLeft) (Utilities|Array|MakeArray 3 6 17 2 13 18 7 16 20 12 19 21)))
              (if (Class|KismetMathLibrary|NotEqualExactlyVectorVector (Variables|Backend|GetCenterRight) (Variables|Backend|GetCenterTrackRight))
                (CallFunction|UpdateVertexPostionThroughCenter (Variables|Backend|GetCenterRight) (Variables|Backend|GetCenterTrackRight) (Utilities|Array|MakeArray 0 5 10 1 9 14 4 11 23 8 15 22)))
              (if (Class|KismetMathLibrary|NotEqualExactlyVectorVector (Variables|Backend|GetCenterFront) (Variables|Backend|GetCenterTrackFront))
                (CallFunction|UpdateVertexPostionThroughCenter (Variables|Backend|GetCenterFront) (Variables|Backend|GetCenterTrackFront) (Utilities|Array|MakeArray 3 6 17 0 5 10 4 11 23 7 16 20)))
              (if (Class|KismetMathLibrary|NotEqualExactlyVectorVector (Variables|Backend|GetCenterBack) (Variables|Backend|GetCenterTrackBack))
                (CallFunction|UpdateVertexPostionThroughCenter (Variables|Backend|GetCenterBack) (Variables|Backend|GetCenterTrackBack) (Utilities|Array|MakeArray 2 13 18 1 9 14 8 15 22 12 19 21)))
              (if (Class|KismetMathLibrary|NotEqualExactlyVectorVector (Variables|Backend|GetCenterBottom) (Variables|Backend|GetCenterTrackBottom))
                (CallFunction|UpdateVertexPostionThroughCenter (Variables|Backend|GetCenterBottom) (Variables|Backend|GetCenterTrackBottom) (Utilities|Array|MakeArray 7 16 20 4 11 23 8 15 22 12 19 21))))))
        (:then_1
          (bind _caluclated_centerposition_7 (CallFunction|UpdateCenterPosition 0 2))
          (Variables|Backend|SetCenterTop _caluclated_centerposition_7)
          (bind _caluclated_centerposition_8 (CallFunction|UpdateCenterPosition 2 7))
          (Variables|Backend|SetCenterLeft _caluclated_centerposition_8)
          (bind _caluclated_centerposition_9 (CallFunction|UpdateCenterPosition 0 8))
          (Variables|Backend|SetCenterRight _caluclated_centerposition_9)
          (bind _caluclated_centerposition_10 (CallFunction|UpdateCenterPosition 7))
          (Variables|Backend|SetCenterFront _caluclated_centerposition_10)
          (bind _caluclated_centerposition_11 (CallFunction|UpdateCenterPosition 2 8))
          (Variables|Backend|SetCenterBack _caluclated_centerposition_11)
          (bind _caluclated_centerposition_12 (CallFunction|UpdateCenterPosition 7 8))
          (Variables|Backend|SetCenterBottom _caluclated_centerposition_12))
        (:then_2
          (Class|ProceduralMeshComponent|CreateMeshSectionLinearColor (Variables|Default|GetProceduralMesh) 0 (Variables|Backend|GetVertices) (Variables|Backend|GetTriangles) (Variables|Backend|GetNormals) (Variables|Backend|GetUV) 0 0 0 0 (Variables|Backend|GetTangents) true false)
          (Rendering|Material|SetMaterial (Variables|Default|GetProceduralMesh) 0 (Variables|Default|GetMaterial))
          (Variables|Backend|SetCenterTrackTop (Variables|Backend|GetCenterTop))
          (Variables|Backend|SetCenterTrackLeft (Variables|Backend|GetCenterLeft))
          (Variables|Backend|SetCenterTrackRight (Variables|Backend|GetCenterRight))
          (Variables|Backend|SetCenterTrackFront (Variables|Backend|GetCenterFront))
          (Variables|Backend|SetCenterTrackBack (Variables|Backend|GetCenterBack))
          (Variables|Backend|SetCenterTrackBottom (Variables|Backend|GetCenterBottom)))))))

(fn UpdateVertexPostionThroughCenter
  (params (MovingCenter :type Vector) (TrackCenter' :type Vector) (VertexIndexArray :type Array%20of%20Integers))
  (bind _vertices (Variables|Backend|GetVertices))
  (for _array_element VertexIndexArray
    (Utilities|Array|SetArrayElem _vertices _array_element (+ (Utilities|Array|Get(acopy) _vertices _array_element) (- MovingCenter TrackCenter')))))

(fn UpdateCenterPosition
  (params (Vertex1 :type Integer) (Vertex2 :type Integer))
  (bind _vertices (Variables|Backend|GetVertices))
  (bind _output (Utilities|Array|Get(acopy) _vertices Vertex1))
  (bind _output_2 (Utilities|Array|Get(acopy) _vertices Vertex2))
  (return (Math|Vector|MakeVector (/ (+ (.x _output) (.x _output_2)) 2.0) (/ (+ (.y _output) (.y _output_2)) 2.0) (/ (+ (.z _output) (.z _output_2)) 2.0))))