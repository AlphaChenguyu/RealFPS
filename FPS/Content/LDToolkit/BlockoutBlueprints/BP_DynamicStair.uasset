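; Blockout tool actor that procedurally generates a linear staircase with Geometry Script.
; On each mesh rebuild, it derives step width, height and depth from the box size and step count, with optional floating steps.
; It then remaps material IDs and applies a single material.
; A bake event copies the generated dynamic mesh into a target static mesh asset when one is valid.
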(event Custom|Bake%20To%20Static%20Mesh
  (bind _returnvalue (DynamicMeshComponent|GetDynamicMesh (Variables|DynamicMeshActor|GetDynamicMeshComponent)))
  (bind _target_mesh (Variables|Default|GetTarget%20Mesh)
    (:then
      (GeometryScript|StaticMesh|CopyMeshtoStaticMesh :FromDynamicMesh _returnvalue :ToStaticMeshAsset _target_mesh :Debug 0))
    (:else)))

(event Events|EventOnRebuildGeneratedMesh
  (params (TargetMesh :type Dynamic%20Mesh%20Object%20Reference))
  (bind _boxsize (Variables|Default|GetBoxSize))
  (bind _num_steps (Variables|Default|GetNum%20Steps))
  (bind _output_get (Variables|Default|SetDynamic%20Mesh TargetMesh))
  (bind _returnvalue (Class|GeometryScriptLibraryMeshPrimitiveFunctions|AppendLinearStairs :TargetMesh _output_get :Transform (Math|Transform|MakeTransform (Math|Vector|MakeVector 0.0 (/ (.y (Variables|Default|GetBoxSize)) 2.0) 0.0) "0, 0, 0" "1.000000,1.000000,1.000000") :StepWidth (.y _boxsize) :StepHeight (/ (.z _boxsize) _num_steps) :StepDepth (/ (.x _boxsize) _num_steps) :NumSteps _num_steps :bFloating (Variables|Default|GetFloating) :Debug 0))
  (GeometryScript|Materials|RemapMaterialIDs _returnvalue 0 0 0)
  (Class|DynamicMeshComponent|ConfigureMaterialSet (Variables|DynamicMeshActor|GetDynamicMeshComponent) (Utilities|Array|MakeArray (Variables|Default|GetMaterial))))

(fn ConstructionScript)