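; BP_LDToolParent is a base actor Blueprint for a level design toolkit, providing an optional text description and in-game hiding.
; Its construction script toggles the description component hierarchy's visibility from a flag and writes the ObjectDescription text into it.
; It also applies the HiddenInGame setting to the root and all its children.
; The event graph holds only disabled default events, so all behavior runs at construction time.
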(event EventBeginPlay)

(event Collision|EventActorBeginOverlap
  (params (OtherActor :type Actor%20Object%20Reference)))

(event EventTick
  (params (DeltaSeconds :type Float%20%28single-precision%29)))

(fn ConstructionScript
  (CallFunction|SetDescriptionVisibility)
  (CallFunction|SetHiddeninGame))

(fn SetDescriptionVisibility
  (if (Variables|Default|Visibility|GetDescriptionVisibile)
    (Rendering|SetVisibility (Variables|Default|GetDescriptionOwner) true true)
    (else
      (Rendering|SetVisibility (Variables|Default|GetDescriptionOwner) false true)))
  (Rendering|Components|TextRender|SetText (Variables|Default|GetDescription) (Variables|Default|GetObjectDescription)))

(fn SetHiddeninGame
  (Development|SetHiddeninGame (Variables|Default|GetDefaultSceneRoot) (Variables|Default|Visibility|GetHiddenInGame) true))