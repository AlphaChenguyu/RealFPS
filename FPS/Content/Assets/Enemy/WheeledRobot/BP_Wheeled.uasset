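; Wheeled robot enemy character that chases and shoots the player, with an overhead state widget and death handling.
; Pawn sensing and incoming damage feed blackboard keys for target, chase, attack and death, with attack range rechecked every tick once damaged.
; AttackPlayer turns toward the player with clamped pitch, plays a montage and spawns a bullet.
; Damage spawns Niagara numbers; death plays an effect, notifies player and game mode, and destroys the actor.
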(event OnSeePawn(PawnSensing)
  (params (Pawn :type Pawn%20Object%20Reference))
  ;[0.15 0.15 0.15 0.5] 视觉感知Pawn
  (bind _asbp_third_person_character (Utilities|Casting|CastToBP_ThirdPersonCharacter Pawn))
  (AI|Components|Blackboard|SetValueasObject (AI|GetBlackboard 0) (Utilities|Name|MakeLiteralName "AttackTarget") _asbp_third_person_character)
  ;[0.15 0.15 0.15 0.5] 距离小于 则BB设置为攻击状态
  (AI|Components|Blackboard|SetValueasBool (AI|GetBlackboard 0) (Utilities|Name|MakeLiteralName "IsAttack") (< (Math|Vector|VectorLength (- (Transformation|GetActorLocation) (Transformation|GetActorLocation (Game|GetPlayerCharacter 0)))) 1.5e+03)))

(event Custom|AttackPlayer
  (bind _returnvalue (Game|GetPlayerCharacter 0))
  (bind _returnvalue_2 (Transformation|GetActorLocation))
  (bind _returnvalue_3 (Transformation|GetActorLocation _returnvalue))
  (bind _returnvalue_4 (- _returnvalue_3 "0.000000,0.000000,50.000000"))
  (bind _returnvalue_5 (Math|Rotator|FindLookatRotation _returnvalue_2 _returnvalue_4))
  ;[0.15 0.15 0.15 0.5] 攻击玩家逻辑
  (bind _asbp_third_person_character (Utilities|Casting|CastToBP_ThirdPersonCharacter (Game|GetPlayerCharacter 0)))
  (if (and (> (Variables|Default|GetHealth) 0.0) (> (Variables|/Game/Assets/BluePrint/BP_ThirdPersonCharacter.BP_ThirdPersonCharacter_C|GetHealth _asbp_third_person_character) 0.0))
    (Transformation|SetActorRotation (Math|Rotator|MakeRotator 0.0 (Math|Float|Clamp(Float) (.pitch _returnvalue_5) -5e+01 75.0) (.yaw _returnvalue_5)))
    (Animation|PlayAnimMontage "/Game/Assets/Enemy/WheeledRobot/Anim/Anim_SciFiDroid01_Shoot2_Montage.Anim_SciFiDroid01_Shoot2_Montage" 0.3 "None")
    (Game|SpawnActorfromClass "/Game/Assets/Enemy/BP_EnemyBullet.BP_EnemyBullet_C" (Transformation|GetWorldTransform (Variables|Default|GetBullet%20Spawn%20Point)) "Undefined" "MultiplyWithRoot" self 0)))

(event EventBeginPlay
  (Variables|/Script/Engine.CharacterMovementComponent|SetMaxWalkSpeed (Variables|Character|GetCharacterMovement) 3e+02)
  (Variables|Default|SetMaxHealth (Variables|Default|GetHealth))
  (bind _aswheeled_enemy_states (Utilities|Casting|CastToWheeled_EnemyStates (UserInterface|GetWidget (Variables|Default|GetWidget))))
  (Variables|/Game/Assets/UI/Wheeled_EnemyStates.Wheeled_EnemyStates_C|SetEnemy _aswheeled_enemy_states self)
  (bind _asbp_third_person_character (Utilities|Casting|CastToBP_ThirdPersonCharacter (Game|GetPlayerCharacter 0)))
  (Variables|Default|SetPlayerRef _asbp_third_person_character))

(event EventTakeDamage
  (params (DamageAmount :type Float%20%28double-precision%29))
  (bind _returnvalue (Transformation|GetActorLocation))
  (bind (_x _y _z) (Math|Vector|BreakVector _returnvalue))
  ;[0.15 0.15 0.15 0.5] GetDamaged
  (if (> (Variables|Default|GetHealth) 0.0)
    (bind _returnvalue_2 (Niagara|SpawnSystematLocation "/Game/Assets/VFX/DamageNumber.DamageNumber" (+ (Transformation|GetActorLocation) "0.000000,0.000000,100.000000")))
    (Class|NiagaraComponent|SetVariableInt _returnvalue_2 "Number" (Math|Float|Truncate DamageAmount))
    ;;[0.15 0.15 0.15 0.5] SetBlackBoard
    (bind _output_get (Variables|Default|SetIsDamaged true))
    (AI|Components|Blackboard|SetValueasBool (AI|GetBlackboard 0) (Utilities|Name|MakeLiteralName "IsChase") _output_get)
    (Variables|/Script/Engine.CharacterMovementComponent|SetMaxWalkSpeed (Variables|Character|GetCharacterMovement) (Variables|Default|GetChaseSpeed))
    (bind _output_get_2 (Variables|Default|SetHealth (- (Variables|Default|GetHealth) DamageAmount)))
    (if (<= _output_get_2 0.0)
      (Default|HandleEnemyKilled (Variables|Default|GetPlayerRef))
      (Variables|Default|SetHealth 0.0)
      (Niagara|SpawnSystematLocation "/Game/Basic_VFX/Niagara/NS_Basic_2.NS_Basic_2" (Math|Vector|MakeVector _x _y (+ _z 5e+01)) "0, 0, 0" "2.000000,2.000000,2.000000")
      (AI|Components|Blackboard|SetValueasBool (AI|GetBlackboard 0) (Utilities|Name|MakeLiteralName "IsDead") true)
      (Utilities|FlowControl|Delay 1.0)
      (Components|DestroyComponent (Variables|Default|GetWidget))
      (Actor|DestroyActor)
      (bind _asbp_fpsgame_mode (Utilities|Casting|CastToBP_FPSGameMode (Game|GetGameMode)))
      (Default|EnemyKilled _asbp_fpsgame_mode))))

(event EventTick
  (params (DeltaSeconds :type Float%20%28single-precision%29))
  ;[0.15 0.15 0.15 0.5] 实时判断收到攻击
  (if (Variables|Default|GetIsDamaged)
    ;[0.15 0.15 0.15 0.5] 距离小于 则BB设置为攻击状态
    (AI|Components|Blackboard|SetValueasBool (AI|GetBlackboard 0) (Utilities|Name|MakeLiteralName "IsAttack") (< (Math|Vector|VectorLength (- (Transformation|GetActorLocation) (Transformation|GetActorLocation (Game|GetPlayerCharacter 0)))) 1.5e+03))))

(fn ConstructionScript)