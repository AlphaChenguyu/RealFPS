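; Base Mutant enemy character that chases and punches the player and dies when its health runs out.
; Pawn sensing, damage and a distance check on Tick feed target, chase, attack and death flags to the AI Blackboard.
; Taking damage shows numbers on its widget and raises walk speed, while punching halts movement.
; Death plays a montage, notifies the game mode of the kill and destroys the actor.
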(event OnSeePawn(PawnSensing)
  (params (Pawn :type Pawn%20Object%20Reference))
  ;[0.15 0.15 0.15 0.5] 视觉感知Pawn
  (bind _asbp_third_person_character (Utilities|Casting|CastToBP_ThirdPersonCharacter Pawn))
  (AI|Components|Blackboard|SetValueasObject (AI|GetBlackboard 0) (Utilities|Name|MakeLiteralName "AttackTarget") _asbp_third_person_character)
  ;[0.15 0.15 0.15 0.5] 距离小于200则BB设置为攻击状态
  (AI|Components|Blackboard|SetValueasBool (AI|GetBlackboard 0) (Utilities|Name|MakeLiteralName "IsAttack") (< (Math|Vector|VectorLength (- (Transformation|GetActorLocation) (Transformation|GetActorLocation (Game|GetPlayerCharacter 0)))) 2e+02)))

(event Custom|GetDamaged
  (params (damageValue :type Float%20%28double-precision%29))
  ;[0.15 0.15 0.15 0.5] GetDamaged
  (if (> (Variables|Default|GetHealth) 0.0)
    ;;[0.15 0.15 0.15 0.5] DisplayDamgaeNumber
    (bind _asmutant_enemy_states (Utilities|Casting|CastToMutant_EnemyStates (UserInterface|GetWidget (Variables|Default|GetWidget))))
    (Default|DisplayNumber _asmutant_enemy_states damageValue)
    ;;[0.15 0.15 0.15 0.5] SetBlackBoard
    (bind _output_get (Variables|Default|SetIsDamaged true))
    (AI|Components|Blackboard|SetValueasBool (AI|GetBlackboard 0) (Utilities|Name|MakeLiteralName "IsChase") _output_get)
    (Variables|/Script/Engine.CharacterMovementComponent|SetMaxWalkSpeed (Variables|Character|GetCharacterMovement) 4e+02)
    (bind _output_get_2 (Variables|Default|SetHealth (- (Variables|Default|GetHealth) damageValue)))
    (if (<= _output_get_2 0.0)
      (Variables|Default|SetHealth 0.0)
      (Animation|PlayAnimMontage "/Game/Assets/Enemy/Mutant/Animations/Mutant_Dying_Montage.Mutant_Dying_Montage" 1.0 "None")
      (AI|Components|Blackboard|SetValueasBool (AI|GetBlackboard 0) (Utilities|Name|MakeLiteralName "IsDead") true)
      (Utilities|FlowControl|Delay 1.0)
      (Components|DestroyComponent (Variables|Default|GetWidget))
      (bind _asbp_fpsgame_mode (Utilities|Casting|CastToBP_FPSGameMode (Game|GetGameMode)))
      (Default|EnemyKilled _asbp_fpsgame_mode)
      (Utilities|FlowControl|Delay 2.0)
      (Actor|DestroyActor))))

(event Custom|AttackPlayer
  (bind _charactermovement (Variables|Character|GetCharacterMovement))
  ;[0.15 0.15 0.15 0.5] 攻击玩家逻辑
  (bind _asbp_third_person_character (Utilities|Casting|CastToBP_ThirdPersonCharacter (Game|GetPlayerCharacter 0)))
  (if (and (> (Variables|Default|GetHealth) 0.0) (> (Variables|/Game/Assets/BluePrint/BP_ThirdPersonCharacter.BP_ThirdPersonCharacter_C|GetHealth _asbp_third_person_character) 0.0))
    (bind _returnvalue (Animation|PlayAnimMontage "/Game/Assets/Enemy/Mutant/Animations/Mutant_Punch_Montage.Mutant_Punch_Montage" 1.0 "None"))
    (Variables|/Script/Engine.CharacterMovementComponent|SetMaxWalkSpeed _charactermovement 0.0)
    (Utilities|FlowControl|Delay _returnvalue)
    (Variables|/Script/Engine.CharacterMovementComponent|SetMaxWalkSpeed _charactermovement 4e+02)))

(event Custom|EnemyAttack
  ;[0.15 0.15 0.15 0.5] 攻击后执行玩家受到伤害
  (bind _asbp_third_person_character (Utilities|Casting|CastToBP_ThirdPersonCharacter (Game|GetPlayerCharacter 0)))
  (Default|PlayerGetDamaged _asbp_third_person_character 2e+01))

(event EventBeginPlay
  (Variables|/Script/Engine.CharacterMovementComponent|SetMaxWalkSpeed (Variables|Character|GetCharacterMovement) 2e+02)
  (Variables|Default|SetMaxHealth (Variables|Default|GetHealth))
  (bind _asmutant_enemy_states (Utilities|Casting|CastToMutant_EnemyStates (UserInterface|GetWidget (Variables|Default|GetWidget))))
  (Variables|/Game/Assets/UI/Mutant_EnemyStates.Mutant_EnemyStates_C|SetEnemy _asmutant_enemy_states self))

(event Collision|EventActorBeginOverlap
  (params (OtherActor :type Actor%20Object%20Reference)))

(event EventTick
  (params (DeltaSeconds :type Float%20%28single-precision%29))
  ;[0.15 0.15 0.15 0.5] 实时判断收到攻击
  (if (Variables|Default|GetIsDamaged)
    ;[0.15 0.15 0.15 0.5] 距离小于200则BB设置为攻击状态
    (AI|Components|Blackboard|SetValueasBool (AI|GetBlackboard 0) (Utilities|Name|MakeLiteralName "IsAttack") (< (Math|Vector|VectorLength (- (Transformation|GetActorLocation) (Transformation|GetActorLocation (Game|GetPlayerCharacter 0)))) 2e+02))))

(fn ConstructionScript)