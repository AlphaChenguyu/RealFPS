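; Laser turret enemy that sweeps its base on a timeline until it sees the player or takes damage.
; When alerted, it aims body yaw and sphere pitch, locks them while charging with a Niagara warning beam, then fires a sphere trace that damages the player.
; A timer reset on each sighting clears detection to resume scanning.
; Damage shows numbers on its widget; death notifies the player, spawns an effect and destroys it.
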(event Custom|StartCharging
  ;[0.15 0.15 0.15 0.5] Charging
  (Variables|Default|SetbIsCharging true)
  (Transformation|SetActorRotation (Variables|Default|GetLockedYawRot))
  (Transformation|SetRelativeRotation (Variables|Default|GetSphere) (Variables|Default|GetLockedPitchRot) false false)
  (Niagara|SetNiagaraVariable(Float) (Variables|Default|GetNiagaraAlert) "LaserLength " (+ 1e+02 (Math|Vector|VectorLength (- (Transformation|GetWorldLocation (Variables|Default|GetBase)) (Transformation|GetWorldLocation (Variables|/Script/Engine.Actor|GetRootComponent (Game|GetPlayerCharacter 0)))))))
  (Timeline|ChargingTimeline PlayFromStart
    (:Finished
      (CallFunction|FireLaser)
      (Utilities|FlowControl|Delay 1.5)
      (Variables|Default|SetbIsCharging false)
      (Niagara|SetNiagaraVariable(Float) (Variables|Default|GetNiagaraAlert) "LaserLength " 0.0))))

(event Custom|FireLaser
  (bind _cylinder (Variables|Default|GetCylinder))
  (bind _returnvalue (Transformation|GetWorldLocation _cylinder))
  ;[0.15 0.15 0.15 0.5] Fire and calculate damage
  (Niagara|SetNiagaraVariable(Float) (Variables|Default|GetNiagara) "LaserLength " (+ 1e+02 (Math|Vector|VectorLength (- (Transformation|GetWorldLocation (Variables|Default|GetBase)) (Transformation|GetWorldLocation (Variables|/Script/Engine.Actor|GetRootComponent (Game|GetPlayerCharacter 0)))))))
  (bind _outhit (Collision|SphereTraceByChannel (- _returnvalue (* (Math|Vector|GetUpVector _cylinder) 2e+03)) (+ _returnvalue (* (Math|Vector|GetUpVector _cylinder) 2e+03)) 15.0 "TraceTypeQuery1" false 0 "None"))
  (bind _asbp_third_person_character (Utilities|Casting|CastToBP_ThirdPersonCharacter (.HitActor (Collision|BreakHitResult _outhit))))
  (Default|PlayerGetDamaged _asbp_third_person_character (Variables|Default|GetLaserDamage) self))

(event Custom|HandleSeePawn
  (params (Pawn :type Pawn%20Object%20Reference))
  (Variables|Default|SetIsPlayerDetected true)
  (Utilities|FlowControl|Sequence
    (:then_0
      (bind _yawvalue (Timeline|RotateTimeline Stop)
        (:Update
          (Transformation|SetRelativeRotation (Variables|Default|GetBase) (Math|Rotator|MakeRotator 0.0 0.0 (+ (Variables|Default|GetInitialYaw) _yawvalue)) false false))))
    (:then_1
      (Utilities|Time|SetTimerbyFunctionName 0 "HandleLostSight" (Variables|Default|GetLostSightDelay)))))

(event EventBeginPlay
  (EventDispatchers|BindEventtoOnSeePawn (Variables|Default|GetPawnSensing) (EventDispatchers|CreateEvent :!event Custom|HandleSeePawn))
  (bind _asbp_third_person_character (Utilities|Casting|CastToBP_ThirdPersonCharacter (Game|GetPlayerCharacter 0)))
  (Variables|Default|SetPlayerRef _asbp_third_person_character)
  (Variables|Default|SetMaxHealth (Variables|Default|GetHealth))
  (Variables|Default|SetInitialYaw (.yaw (Variables|/Script/Engine.SceneComponent|GetRelativeRotation (Variables|Default|GetBase))))
  (bind _aslaser_turret_enemy_states (Utilities|Casting|CastToLaserTurret_EnemyStates (UserInterface|GetWidget (Variables|Default|GetWidget))))
  (Variables|/Game/Assets/UI/LaserTurret_EnemyStates.LaserTurret_EnemyStates_C|SetEnemy _aslaser_turret_enemy_states self)
  (bind _yawvalue (Timeline|RotateTimeline PlayFromStart)
    (:Update
      (Transformation|SetRelativeRotation (Variables|Default|GetBase) (Math|Rotator|MakeRotator 0.0 0.0 (+ (Variables|Default|GetInitialYaw) _yawvalue)) false false))))

(event EventTakeDamage
  (params (DamageAmount :type Float%20%28double-precision%29))
  (bind _returnvalue (Transformation|GetActorLocation))
  (bind (_x _y _z) (Math|Vector|BreakVector _returnvalue))
  ;[0.15 0.15 0.15 0.5] GetDamaged
  (if (> (Variables|Default|GetHealth) 0.0)
    (bind _output_get (Variables|Default|SetHealth (- (Variables|Default|GetHealth) DamageAmount)))
    (Variables|Default|SetIsPlayerDetected true)
    (Utilities|FlowControl|Sequence
      (:then_0
        ;;[0.15 0.15 0.15 0.5] DisplayDamgaeNumber
        (bind _aslaser_turret_enemy_states (Utilities|Casting|CastToLaserTurret_EnemyStates (UserInterface|GetWidget (Variables|Default|GetWidget))))
        (Default|DisplayLaserTurretNumber _aslaser_turret_enemy_states DamageAmount)
        (if (<= _output_get 0.0)
          (Variables|Default|SetHealth 0.0)
          (Default|HandleEnemyKilled (Variables|Default|GetPlayerRef))
          (Niagara|SpawnSystematLocation "/Game/Basic_VFX/Niagara/NS_Basic_2.NS_Basic_2" (Math|Vector|MakeVector _x _y (+ _z 1e+02)) "0, 0, 0" "2.000000,2.000000,2.000000")
          (Utilities|FlowControl|Delay 1.0)
          (Actor|DestroyActor)))
      (:then_2
        (bind _yawvalue (Timeline|RotateTimeline Stop)
          (:Update
            (Transformation|SetRelativeRotation (Variables|Default|GetBase) (Math|Rotator|MakeRotator 0.0 0.0 (+ (Variables|Default|GetInitialYaw) _yawvalue)) false false)))))))

(event EventTick
  (params (DeltaSeconds :type Float%20%28single-precision%29))
  (bind _returnvalue (Game|GetPlayerCharacter 0))
  (bind _returnvalue_2 (Transformation|GetActorLocation _returnvalue))
  ;[0.15 0.15 0.15 0.5] Aiming
  (if (Variables|Default|GetIsPlayerDetected)
    (if (not (Variables|Default|GetbIsCharging))
      (bind _output_get (Variables|Default|SetLockedYawRot (Math|Rotator|MakeRotator 0.0 0.0 (.yaw (Math|Rotator|FindLookatRotation (Transformation|GetActorLocation) _returnvalue_2)))))
      (Transformation|SetActorRotation _output_get)
      (bind _output_get_2 (Variables|Default|SetLockedPitchRot (Math|Rotator|MakeRotator 0.0 (.Pitch (Math|Rotator|BreakRotator (Math|Conversions|RotationFromXVector (- _returnvalue_2 (Transformation|GetWorldLocation (Variables|Default|GetSphere)))))) 0.0)))
      (Transformation|SetRelativeRotation (Variables|Default|GetSphere) _output_get_2 false false)
      (CallFunction|StartCharging))
    (else
      (bind _yawvalue (Timeline|RotateTimeline PlayFromStart)
        (:Update
          (Transformation|SetRelativeRotation (Variables|Default|GetBase) (Math|Rotator|MakeRotator 0.0 0.0 (+ (Variables|Default|GetInitialYaw) _yawvalue)) false false))))))

(fn ConstructionScript)

(fn HandleLostSight
  (Variables|Default|SetIsPlayerDetected false))