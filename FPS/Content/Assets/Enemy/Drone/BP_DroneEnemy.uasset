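; Hovering drone enemy that chases any pawn its PawnSensing spots and shoots bullets at it.
; Tick either fires within range or interpolates toward the target at hover height, but does nothing once the drone strays beyond its chase radius from spawn.
; Firing aims below the target's origin, then waits out the cooldown before spawning each bullet.
; Damage shows numbers on a widget and destroys the drone shortly after health runs out.
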(event OnSeePawn(PawnSensing)
  (params (Pawn :type Pawn%20Object%20Reference))
  (Variables|Default|SetTargetActor%20 Pawn))

(event Custom|FireAtTarget
  (Variables|Default|SetbIsOnCooldown true)
  (Transformation|SetActorRotation (Math|Rotator|FindLookatRotation (Transformation|GetActorLocation) (- (Transformation|GetActorLocation (Variables|Default|GetTargetActor%20)) "0.000000,0.000000,100.000000")))
  (Utilities|FlowControl|Delay (Variables|Default|GetFireCooldown))
  (Game|SpawnActorfromClass "/Game/Assets/Enemy/Drone/BP_DroneBullet.BP_DroneBullet_C" (Transformation|GetWorldTransform (Variables|组件|GetProjectileSpawnPoint)) "Undefined" "MultiplyWithRoot" 0 0)
  (Variables|Default|SetbIsOnCooldown false))

(event Custom|GetDamaged
  (params (damageValue :type Float%20%28double-precision%29))
  ;[0.15 0.15 0.15 0.5] GetDamaged
  (if (> (Variables|Default|GetHealth) 0.0)
    (bind _output_get (Variables|Default|SetHealth (- (Variables|Default|GetHealth) damageValue)))
    ;;[0.15 0.15 0.15 0.5] DisplayDamgaeNumber
    (bind _asdrone_enemy_states (Utilities|Casting|CastToDrone_EnemyStates (UserInterface|GetWidget (Variables|组件|GetWidget))))
    (Default|DisplayDroneNumber _asdrone_enemy_states damageValue)
    (if (<= _output_get 0.0)
      (Variables|Default|SetHealth 0.0)
      (Utilities|FlowControl|Delay 1.0)
      (Actor|DestroyActor))))

(event Custom|MoveToTarget
  (bind _targetactor_ (Variables|Default|GetTargetActor%20))
  (bind _returnvalue (Transformation|GetActorLocation _targetactor_))
  (bind (_x _y) (Math|Vector|BreakVector _returnvalue))
  (Transformation|SetActorRotation (Math|Rotator|FindLookatRotation (Transformation|GetActorLocation) (Transformation|GetActorLocation (Variables|Default|GetTargetActor%20))))
  (Transformation|SetActorLocation (Math|Interpolation|VInterpTo (Transformation|GetActorLocation) (Math|Vector|MakeVector _x _y (Variables|Default|GetHoverZ)) (Utilities|Time|GetWorldDeltaSeconds) (Variables|Default|GetMoveSpeed)) false false))

(event EventBeginPlay
  (Variables|Default|SetSpawnLocation (Transformation|GetActorLocation))
  (Variables|Default|SetMaxHealth (Variables|Default|GetHealth))
  (bind _asdrone_enemy_states (Utilities|Casting|CastToDrone_EnemyStates (UserInterface|GetWidget (Variables|组件|GetWidget))))
  (Variables|/Game/Assets/UI/Drone_EnemyStates.Drone_EnemyStates_C|SetEnemy _asdrone_enemy_states self))

(event EventTick
  (params (DeltaSeconds :type Float%20%28single-precision%29))
  (bind _targetactor_ (Variables|Default|GetTargetActor%20))
  (Utilities|IsValid _targetactor_
    (:Is%20Valid
      (if (<= (Math|Vector|VectorLength (- (Transformation|GetActorLocation) (Variables|Default|GetSpawnLocation))) (Variables|Default|GetChaseRadius))
        (if (and (<= (Math|Vector|VectorLength (- (Transformation|GetActorLocation _targetactor_) (Transformation|GetActorLocation))) (Variables|Default|GetFireRange)) (> (Variables|Default|GetHealth) 0.0))
          (if (not (Variables|Default|GetbIsOnCooldown))
            (CallFunction|FireatTarget))
          (else
            (CallFunction|MovetoTarget)))))))

(fn ConstructionScript)