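; BP_PickupItem is a weapon pickup that gives the player a rifle or shotgun on interaction.
; The construction script applies ItemModel to the Item skeletal mesh.
; StartInteract caches the player character, waits briefly, then runs the WeaponSlot macro, which uses Slot to snap Item to a back or low socket and set that weapon's reference and flag.
; It then prints a message and disables the actor's collision.
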(event EventStartInteract
  (bind _asbp_third_person_character (Utilities|Casting|CastToBP_ThirdPersonCharacter (Game|GetPlayerCharacter 0)))
  (Variables|Default|SetCharacter%20Ref _asbp_third_person_character)
  (Utilities|FlowControl|Delay 0.1)
  (Utilities|WeaponSlot
    (:Out
      (Development|PrintString "Weapon Pickedup")
      (Collision|SetActorEnableCollision false))))

(fn ConstructionScript
  (Components|SkeletalMesh|SetSkeletalMeshAsset (Variables|Default|GetItem) (Variables|Default|GetItemModel)))