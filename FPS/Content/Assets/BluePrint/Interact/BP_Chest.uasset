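; BP_Chest is an interactable chest that opens a bonus selection screen for the first player.
; On StartInteract it creates WBP_BonusSelect with a reference to itself, unless one is already open, then switches to UI-only input and shows the cursor.
; The widget's exit event removes it, restores game-only input, hides the cursor and clears the reference so the chest can open it again.
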(event Custom|OnBonusUIExit
  (bind _returnvalue (Game|GetPlayerController 0))
  (Widget|RemovefromParent (stale EventStartInteract _output_get))
  (Input|SetInputModeGameOnly _returnvalue false)
  (Variables|/Script/Engine.PlayerController|SetbShowMouseCursor _returnvalue false)
  (Variables|Default|SetBonusUIRef 0))

(event EventBeginPlay
  (Input|EnableInput (Game|GetPlayerController 0)))

(event EventStartInteract
  (bind _returnvalue (Game|GetPlayerController 0))
  (Utilities|IsValid (Variables|Default|GetBonusUIRef)
    (:Is%20Not%20Valid
      (bind _returnvalue_2 (UserInterface|CreateWidget "/Game/Assets/UI/WBP_BonusSelect.WBP_BonusSelect_C" _returnvalue self))
      (bind _output_get (Variables|Default|SetBonusUIRef _returnvalue_2))
      (EventDispatchers|BindEventtoOnExitRequested _output_get (delegate Custom|OnBonusUIExit))
      (UserInterface|Viewport|AddtoViewport _output_get 0)
      (Input|SetInputModeUIOnly _returnvalue _output_get "DoNotLock" false)
      (Variables|/Script/Engine.PlayerController|SetbShowMouseCursor _returnvalue true))))

(fn ConstructionScript)