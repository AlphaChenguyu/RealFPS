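; Toxic pool trap that damages the third-person player character and launches it upward when it enters the overlap box.
; The construction script randomizes the pool's width and length at a fixed thin height, then scales and offsets the cube mesh and trigger box to match and applies the material.
; Damage is applied once per overlap begin, despite the DamagePerSecond name, with no tick or timer.
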(event OnComponentBeginOverlap(Box)
  (params (OverlappedComponent :type Primitive%20Component%20Object%20Reference) (OtherActor :type Actor%20Object%20Reference) (OtherComp :type Primitive%20Component%20Object%20Reference) (OtherBodyIndex :type Integer) (bFromSweep :type Boolean) (SweepResult :type Hit%20Result%20Structure%20%28by%20ref%29))
  (bind _asbp_third_person_character (Utilities|Casting|CastToBP_ThirdPersonCharacter OtherActor))
  (Default|PlayerGetDamaged _asbp_third_person_character (Variables|Default|GetDamagePerSecond) self)
  (Character|LaunchCharacter _asbp_third_person_character (Math|Vector|MakeVector 0.0 0.0 (Variables|Default|GetForce)) false false))

(event EventBeginPlay)

(event Collision|EventActorBeginOverlap
  (params (OtherActor :type Actor%20Object%20Reference)))

(event EventTick
  (params (DeltaSeconds :type Float%20%28single-precision%29)))

(fn ConstructionScript
  (|CallParentFunction)
  (Utilities|FlowControl|Sequence
    (:then_0
      ;[0.15 0.15 0.15 0.5] Set random boundary
      (bind _output_get (Variables|Default|SetCorner (Math|Vector|MakeVector (Math|Random|RandomFloatinRange 5e+02 1e+03) (Math|Random|RandomFloatinRange 5e+02 1e+03) 1e+01)))
      ;[1 1 1] Set the scale of the box based on the corner variable
      (Transformation|SetWorldScale3D (Variables|Default|GetCube) (/ _output_get 100)))
    (:then_1
      ;[1 1 1] Set the position of the box to fit with the corner variable
      (Transformation|SetRelativeLocation (Variables|Default|GetCube) (/ (Variables|Default|GetCorner) 2) false false))
    (:then_2
      ;[1 1 1] Set the material of the box
      (Rendering|Material|SetMaterial (Variables|Default|GetCube) 0 (Variables|Default|GetMain%20Color)))))