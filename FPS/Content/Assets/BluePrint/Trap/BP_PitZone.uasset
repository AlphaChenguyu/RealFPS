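; BP_PitZone is a trap zone, tracked as gas, that deals repeated damage to a BP_ThirdPersonCharacter inside its box.
; On BeginPlay a timeline drives the Niagara Progress parameter, at a GrowSpeed rate set in the construction script.
; Box overlap deals damage immediately, then starts a looping named timer that repeats it every DamageInterval.
; An IsInGas flag blocks re-triggering, and end overlap resets it and clears the timer.
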(event OnComponentBeginOverlap(Box)
  (params (OverlappedComponent :type Primitive%20Component%20Object%20Reference) (OtherActor :type Actor%20Object%20Reference) (OtherComp :type Primitive%20Component%20Object%20Reference) (OtherBodyIndex :type Integer) (bFromSweep :type Boolean) (SweepResult :type Hit%20Result%20Structure%20%28by%20ref%29))
  (bind _asbp_third_person_character (Utilities|Casting|CastToBP_ThirdPersonCharacter OtherActor))
  (if (not (Variables|Default|GetbIsInGas))
    (Variables|Default|SetbIsInGas true)
    (Default|PlayerGetDamaged _asbp_third_person_character (Variables|Default|GetDamagePerSecond) self)
    (bind _returnvalue (Utilities|Time|SetTimerbyFunctionName 0 "ApplyLoopDamage" (Variables|Default|GetDamageInterval) true))
    (Variables|Default|SetDamageTimerHandle _returnvalue)))

(event OnComponentEndOverlap(Box)
  (params (OverlappedComponent :type Primitive%20Component%20Object%20Reference) (OtherActor :type Actor%20Object%20Reference) (OtherComp :type Primitive%20Component%20Object%20Reference) (OtherBodyIndex :type Integer))
  (Utilities|Casting|CastToBP_ThirdPersonCharacter OtherActor)
  (Variables|Default|SetbIsInGas false)
  (Utilities|Time|ClearTimerbyFunctionName 0 "ApplyLoopDamage"))

(event Custom|ApplyLoopDamage
  (Default|PlayerGetDamaged (stale OnComponentBeginOverlap(Box) _asbp_third_person_character) (Variables|Default|GetDamagePerSecond) self))

(event EventBeginPlay
  (bind _newtrack_0 (Timeline|Timeline Play)
    (:Update
      (Niagara|SetNiagaraVariable(Float) (Variables|Default|GetNiagara) "Progress" _newtrack_0))))

(event Collision|EventActorBeginOverlap
  (params (OtherActor :type Actor%20Object%20Reference)))

(fn ConstructionScript
  (Components|Timeline|SetPlayRate (Variables|Default|GetTimeline) (Variables|Default|GetGrowSpeed)))