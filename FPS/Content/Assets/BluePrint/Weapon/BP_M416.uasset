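; M416 rifle weapon Blueprint that handles firing and reloading for its owning character.
; FireBullet spawns a muzzle bullet aimed via a debug-drawn screen-center trace, which itself applies damage and hitmarkers to BPI_Damageable actors and pushes physics objects.
; Reload plays rifle and character animations, then broadcasts completion.
; UpdateReloadAmmo simply resets CurrentAmmo to TotalAmmo; FireBullet consumes no ammo here, and clip-and-reserve math is left disconnected.
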(event Custom|SetOwningCharacter
  (params (character :type BP%20Third%20Person%20Character%20Object%20Reference))
  (Variables|Default|SetOwningCharacter character))

(event EventUpdateReloadAmmo
  (Variables|Ammo|SetCurrentAmmo (Variables|Ammo|GetTotalAmmo)))

(event EventFireBullet
  (bind _returnvalue (Viewport|GetViewportSize))
  (bind _returnvalue_2 (Game|GetPlayerController 0))
  (bind _owningcharacter (Variables|Default|GetOwningCharacter))
  (bind _rifle_damage (Variables|Default|GetRifle%20Damage))
  (bind _returnvalue_3 (/ _returnvalue 2.0))
  (bind _rifle (Variables|/Game/Assets/BluePrint/BP_ThirdPersonCharacter.BP_ThirdPersonCharacter_C|GetRifle _owningcharacter))
  (bind (_worldposition _worlddirection) (Class|GameplayStatics|DeprojectScreentoWorld _returnvalue_2 _returnvalue_3))
  (bind _returnvalue_4 (* _worlddirection 5e+03))
  (bind _returnvalue_5 (+ _worldposition _returnvalue_4))
  (Components|Animation|PlayAnimation _rifle "/Game/MilitaryWeapDark/Weapons/Anims/Fire_Rifle_W.Fire_Rifle_W" false)
  (bind _returnvalue_6 (Game|SpawnActorfromClass "/Game/Assets/BluePrint/Weapon/BP_RifleBullet.BP_RifleBullet_C" (Transformation|GetSocketTransform _rifle "MuzzleFlash" "RTS_World") "Undefined" "MultiplyWithRoot" 0 0))
  (bind (_outhit _returnvalue_7) (Collision|LineTraceByChannel _worldposition _returnvalue_5 "TraceTypeQuery3" true 0 "ForDuration" true "(R=1.000000,G=0.000000,B=0.000000,A=1.000000)" "(R=0.000000,G=1.000000,B=0.000000,A=1.000000)" 5e+01))
  (Default|SetVelocity _returnvalue_6 (select _returnvalue_7 (.Location (Collision|BreakHitResult _outhit)) _returnvalue_5))
  (Utilities|FlowControl|Sequence
    (:then_0
      (if (Utilities|DoesObjectImplementInterface (.HitActor (Collision|BreakHitResult _outhit)) "/Game/Assets/BluePrint/Interface/BPI_Damageable.BPI_Damageable_C")
        (Default|ShowHitmarker (Variables|/Game/Assets/BluePrint/BP_ThirdPersonCharacter.BP_ThirdPersonCharacter_C|GetMainUI (Variables|Default|GetOwningCharacter)))
        (Class|BPIDamageable|TakeDamage(Message) (.HitActor (Collision|BreakHitResult _outhit)) _rifle_damage)
        (Game|Damage|ApplyPointDamage (.HitActor (Collision|BreakHitResult _outhit)) _rifle_damage (.Location (Collision|BreakHitResult _outhit)) _outhit 0 0 "/Game/BossAIToolkit/Blueprints/DamageTypes/BP_DamageType_Default.BP_DamageType_Default_C")))
    (:then_1
      (if (Physics|IsSimulatingPhysics (.HitComponent (Collision|BreakHitResult _outhit)) "None")
        (Physics|AddImpulseatLocation (.HitComponent (Collision|BreakHitResult _outhit)) "1000.000000,1000.000000,1000.000000" "0, 0, 0" "None")))))

(event EventReload
  (if (not (Math|Boolean|ORBoolean (== (Variables|Ammo|GetCurrentAmmo) (Variables|Ammo|GetTotalAmmo)) (Variables|Default|GetIsReloading?) (Variables|/Game/Assets/BluePrint/BP_ThirdPersonCharacter.BP_ThirdPersonCharacter_C|GetIsDead (Variables|Default|GetOwningCharacter))))
    (Variables|Default|SetIsReloading? true)
    (Components|Animation|PlayAnimation (Variables|/Game/Assets/BluePrint/BP_ThirdPersonCharacter.BP_ThirdPersonCharacter_C|GetRifle (Variables|Default|GetOwningCharacter)) "/Game/MilitaryWeapDark/Weapons/Anims/Prone_Reload_Rifle_W.Prone_Reload_Rifle_W" false)
    (Animation|Montage|PlayMontage (Variables|/Script/Engine.Character|GetMesh (Variables|Default|GetOwningCharacter)) "/Game/Assets/Animation/UE5_Reload_Rifle_Ironsights_Montage.UE5_Reload_Rifle_Ironsights_Montage" 1.0 0.0 "" false
      (:OnCompleted
        (Variables|Default|SetIsReloading? false)
        (Default|CallOnRifleReload)))))

(fn ConstructionScript)