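; Rocket projectile that flies at fixed speed toward a target position and explodes on impact.
; On hit it spawns and triggers a BP_AOE_Explosion, pushes physics-simulating hit components, then destroys itself after a short delay.
; Explosion overlaps call back into DealDamage, which shows the player's hitmarker and damages BPI_Damageable actors via both interface message and unblockable point damage, using player 0's RocketDamage.
; DealDamage destroys the rocket after damaging an actor.
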(event OnComponentHit(HitBox)
  (params (HitComponent :type Primitive%20Component%20Object%20Reference) (OtherActor :type Actor%20Object%20Reference) (OtherComp :type Primitive%20Component%20Object%20Reference) (NormalImpulse :type Vector :default "0, 0, 0") (Hit :type Hit%20Result%20Structure%20%28by%20ref%29))
  (bind (_bblockinghit _binitialoverlap _time _distance _location _impactpoint _normal _impactnormal _physmat _hitactor _hitcomponent) (Collision|BreakHitResult Hit))
  (bind _returnvalue (Game|SpawnActorfromClass "/Game/Assets/BluePrint/AOE/BP_AOE_Explosion.BP_AOE_Explosion_C" (Math|Transform|MakeTransform _location "0, 0, 0" "1.000000,1.000000,1.000000") "Undefined" "MultiplyWithRoot" 0 false true 0))
  (Utilities|FlowControl|Sequence
    (:then_0
      (EventDispatchers|AssignOnAOEOverlapActor _returnvalue (delegate Custom|Deal%20Damage))
      (Default|Trigger _returnvalue)
      (Utilities|FlowControl|Delay 0.2)
      (Actor|DestroyActor))
    (:then_1
      (if (Physics|IsSimulatingPhysics _hitcomponent "None")
        (Physics|AddImpulseatLocation _hitcomponent "1000.000000,1000.000000,1000.000000" "0, 0, 0" "None")))))

(event Custom|SetRocketVelocity
  (params (TargetPos :type Vector))
  (Variables|/Script/Engine.MovementComponent|SetVelocity (Variables|Default|GetProjectileMovement) (* (Math|Vector|Normalize (- TargetPos (Transformation|GetActorLocation))) 5e+03)))

(event Custom|Deal%20Damage
  (params (Actor :type Actor%20Object%20Reference))
  (if (Utilities|DoesObjectImplementInterface Actor "/Game/Assets/BluePrint/Interface/BPI_Damageable.BPI_Damageable_C")
    (bind _asbp_third_person_character (Utilities|Casting|CastToBP_ThirdPersonCharacter (Game|GetPlayerCharacter 0)))
    (Default|ShowHitmarker (Variables|/Game/Assets/BluePrint/BP_ThirdPersonCharacter.BP_ThirdPersonCharacter_C|GetMainUI _asbp_third_person_character))
    (Class|BPIDamageable|TakeDamage(Message) Actor (Variables|/Game/Assets/BluePrint/BP_ThirdPersonCharacter.BP_ThirdPersonCharacter_C|GetRocketDamage _asbp_third_person_character))
    (Game|Damage|ApplyPointDamage Actor (Variables|/Game/Assets/BluePrint/BP_ThirdPersonCharacter.BP_ThirdPersonCharacter_C|GetRocketDamage _asbp_third_person_character) (.Location (Collision|BreakHitResult (stale OnComponentHit(HitBox) Hit))) (stale OnComponentHit(HitBox) Hit) 0 0 "/Game/BossAIToolkit/Blueprints/DamageTypes/BP_DamageType_Unblockable.BP_DamageType_Unblockable_C")
    (Actor|DestroyActor)))

(fn ConstructionScript)