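; Peacekeeper shotgun weapon Blueprint that handles firing and reloading for its owning character.
; FireBullet spawns one bullet at the muzzle, then runs eight random-spread camera traces, each re-aiming that bullet, damaging damageable actors with a hitmarker and pushing physics objects.
; Reload plays weapon and character animations, then signals completion through CallOnShotgunReload.
; UpdateReloadAmmo restores CurrentAmmo to TotalAmmo; the limited-ammo logic is disconnected.
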(event Custom|SetOwningCharacter
  (params (character :type BP%20Third%20Person%20Character%20Object%20Reference))
  (Variables|Default|SetOwningCharacter character))

(event EventFireBullet
  (bind _returnvalue (Viewport|GetViewportSize))
  (bind _returnvalue_2 (Game|GetPlayerController 0))
  (bind _spread (Variables|Default|GetSpread))
  (bind _spread_2 (Variables|Default|GetSpread))
  (bind _spread_3 (Variables|Default|GetSpread))
  (bind _shotgun_damage (Variables|Default|GetShotgun%20Damage))
  (bind _owningcharacter (Variables|Default|GetOwningCharacter))
  (bind _returnvalue_3 (/ _returnvalue 2.0))
  (bind _followcamera (Variables|/Game/Assets/BluePrint/BP_ThirdPersonCharacter.BP_ThirdPersonCharacter_C|GetFollowCamera _owningcharacter))
  (bind _shotgun (Variables|/Game/Assets/BluePrint/BP_ThirdPersonCharacter.BP_ThirdPersonCharacter_C|GetShotgun _owningcharacter))
  (bind (_worldposition _worlddirection) (Class|GameplayStatics|DeprojectScreentoWorld _returnvalue_2 _returnvalue_3))
  (bind _returnvalue_4 (Transformation|GetWorldLocation _followcamera))
  (Components|Animation|PlayAnimation _shotgun "/Game/MilitaryWeapDark/Weapons/Anims/Fire_Shotgun_W.Fire_Shotgun_W" false)
  (bind _returnvalue_5 (Game|SpawnActorfromClass "/Game/Assets/BluePrint/Weapon/BP_ShotgunBullet.BP_ShotgunBullet_C" (Transformation|GetSocketTransform _shotgun "MuzzleFlash" "RTS_World") "Undefined" "MultiplyWithRoot" 0 0))
  (for _index (range 1 8)
    (bind (_outhit _returnvalue_6) (Collision|LineTraceByChannel _returnvalue_4 (+ _returnvalue_4 (* (Math|Vector|GetForwardVector _followcamera) (Variables|Default|GetRange)) (Math|Vector|MakeVector (Math|Random|RandomFloatinRange (* _spread_2 -1.0) _spread_2) (Math|Random|RandomFloatinRange (* _spread_3 -1.0) _spread_3) (Math|Random|RandomFloatinRange (* _spread -1.0) _spread))) "TraceTypeQuery3" true (Utilities|Array|MakeArray _owningcharacter _returnvalue_5) "None"))
    (Default|SetVelocity _returnvalue_5 (select _returnvalue_6 (.Location (Collision|BreakHitResult _outhit)) (+ _worldposition (* _worlddirection 2e+04))))
    (Utilities|FlowControl|Sequence
      (:then_0
        (if (Utilities|DoesObjectImplementInterface (.HitActor (Collision|BreakHitResult _outhit)) "/Game/Assets/BluePrint/Interface/BPI_Damageable.BPI_Damageable_C")
          (Default|ShowHitmarker (Variables|/Game/Assets/BluePrint/BP_ThirdPersonCharacter.BP_ThirdPersonCharacter_C|GetMainUI (Variables|Default|GetOwningCharacter)))
          (Class|BPIDamageable|TakeDamage(Message) (.HitActor (Collision|BreakHitResult _outhit)) _shotgun_damage)
          (Game|Damage|ApplyPointDamage (.HitActor (Collision|BreakHitResult _outhit)) _shotgun_damage (.Location (Collision|BreakHitResult _outhit)) _outhit 0 0 "/Game/BossAIToolkit/Blueprints/DamageTypes/BP_DamageType_Default.BP_DamageType_Default_C")))
      (:then_1
        (if (Physics|IsSimulatingPhysics (.HitComponent (Collision|BreakHitResult _outhit)) "None")
          (Physics|AddImpulseatLocation (.HitComponent (Collision|BreakHitResult _outhit)) "2000.000000,2000.000000,2000.000000" "0, 0, 0" "None"))))))

(event EventReload
  (if (not (Math|Boolean|ORBoolean (== (Variables|Ammo|GetCurrentAmmo) (Variables|Ammo|GetTotal%20Ammo)) (Variables|Default|GetIsReloading?) (Variables|/Game/Assets/BluePrint/BP_ThirdPersonCharacter.BP_ThirdPersonCharacter_C|GetIsDead (Variables|Default|GetOwningCharacter))))
    (Variables|Default|SetIsReloading? true)
    (Components|Animation|PlayAnimation (Variables|/Game/Assets/BluePrint/BP_ThirdPersonCharacter.BP_ThirdPersonCharacter_C|GetShotgun (Variables|Default|GetOwningCharacter)) "/Game/MilitaryWeapDark/Weapons/Anims/Reload_Shotgun_Ironsights_W.Reload_Shotgun_Ironsights_W" false)
    (Animation|Montage|PlayMontage (Variables|/Script/Engine.Character|GetMesh (Variables|Default|GetOwningCharacter)) "/Game/Assets/Animation/UE5_Reload_Shotgun_Ironsights_Montage.UE5_Reload_Shotgun_Ironsights_Montage" (Variables|Default|GetShotgunReloadSpeed) 0.0 "" false
      (:OnCompleted
        (Variables|Default|SetIsReloading? false)
        (Default|CallOnShotgunReload)))))

(event EventUpdateReloadAmmo
  (Variables|Ammo|SetCurrentAmmo (Variables|Ammo|GetTotal%20Ammo)))

(fn ConstructionScript)