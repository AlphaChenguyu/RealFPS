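; BP_RifleBullet is a rifle projectile Blueprint driven by a ProjectileMovement component.
; Its SetVelocity event aims the bullet at a target position by setting a fixed-speed velocity along the normalized direction from its location.
; When its Sphere component registers a hit, it plays a body impact sound, spawns a small metal impact particle effect and destroys itself.
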(event OnComponentHit(Sphere)
  (params (HitComponent :type Primitive%20Component%20Object%20Reference) (OtherActor :type Actor%20Object%20Reference) (OtherComp :type Primitive%20Component%20Object%20Reference) (NormalImpulse :type Vector :default "0, 0, 0") (Hit :type Hit%20Result%20Structure%20%28by%20ref%29))
  (bind _returnvalue (Transformation|GetActorLocation))
  (Audio|PlaySoundatLocation "/Game/MilitaryWeapDark/Sound/Rifle/Wavs/Rifle_ImpactBody01.Rifle_ImpactBody01" _returnvalue "0, 0, 0" 1.0 1.0 0.0 0 0 0 0)
  (Effects|SpawnEmitteratLocation "/Game/MilitaryWeapDark/FX/P_Impact_Metal_Small_01.P_Impact_Metal_Small_01" _returnvalue)
  (Actor|DestroyActor))

(event Custom|SetVelocity
  (params (TargetPos :type Vector))
  (Variables|/Script/Engine.MovementComponent|SetVelocity (Variables|Default|GetProjectileMovement) (* (Math|Vector|Normalize (- TargetPos (Transformation|GetActorLocation))) 8e+03)))

(event EventBeginPlay)

(fn ConstructionScript)