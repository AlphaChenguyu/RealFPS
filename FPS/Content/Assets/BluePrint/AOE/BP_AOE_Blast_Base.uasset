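; BP_AOE_Blast_Base is a base Blueprint for one-shot area-of-effect blasts, extending a parent AOE class with visual and audio feedback.
; When SpawnAoeSphere fires, it runs the parent logic, then spawns BlastEffect attached to the root and plays BlastSound at the actor's location.
; The actor destroys itself when the particle system finishes, or after a short delay if no effect is set, in which case no sound plays.
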(event Custom|SystemFinished
  (params (PSystem :type Particle%20System%20Component%20Object%20Reference))
  ;[0.15 0.15 0.15 0.5] Blast Effects
  (Actor|DestroyActor))

(event EventBeginPlay
  (|CallParentFunction) ; 此节点被禁用，将不会被调用。\n从引脚连出引线来编译功能。
)

(event Collision|EventActorBeginOverlap
  (params (OtherActor :type Actor%20Object%20Reference)))

(event EventTick
  (params (DeltaSeconds :type Float%20%28single-precision%29)))

(event EventSpawnAoeSphere
  (|CallParentFunction)
  ;[0.15 0.15 0.15 0.5] Blast Effects
  (bind _blasteffect (Variables|Default|GetBlastEffect)
    (:then
      (bind _returnvalue (Effects|SpawnEmitterAttached _blasteffect (Variables|Default|GetDefaultSceneRoot) "None"))
      (EventDispatchers|AssignOnSystemFinished _returnvalue (delegate Custom|SystemFinished))
      ;[0.15 0.15 0.15 0.5] Blast Sound
      (bind _blastsound (Variables|Default|GetBlastSound)
        (:then
          (Audio|PlaySoundatLocation _blastsound (Transformation|GetActorLocation) "0, 0, 0" 1.0 1.0 0.0 0 0 0 0))
        (:else)))
    (:else
      (Utilities|FlowControl|Delay 1.0)
      (Actor|DestroyActor))))

(fn ConstructionScript
  (|CallParentFunction))