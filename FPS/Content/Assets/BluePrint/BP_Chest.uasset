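; BP_Chest is an interactable chest that opens a bonus selection UI when the player interacts nearby.
; Box overlaps with BP_ThirdPersonCharacter toggle CanOpen, which gates IA_Interact on input the chest enables for itself at BeginPlay.
; Interacting creates a single WBP_BonusSelect with a chest reference, switching to UI-only input with a visible cursor.
; The widget's OnExitRequested dispatcher removes it, restores game input and clears the reference, allowing reopening.
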(event OnComponentBeginOverlap(Box)
  (params (OverlappedComponent :type Primitive%20Component%20Object%20Reference) (OtherActor :type Actor%20Object%20Reference) (OtherComp :type Primitive%20Component%20Object%20Reference) (OtherBodyIndex :type Integer) (bFromSweep :type Boolean) (SweepResult :type Hit%20Result%20Structure%20%28by%20ref%29))
  (Utilities|Casting|CastToBP_ThirdPersonCharacter OtherActor)
  (Variables|Default|SetCanOpen true))

(event OnComponentEndOverlap(Box)
  (params (OverlappedComponent :type Primitive%20Component%20Object%20Reference) (OtherActor :type Actor%20Object%20Reference) (OtherComp :type Primitive%20Component%20Object%20Reference) (OtherBodyIndex :type Integer))
  (Utilities|Casting|CastToBP_ThirdPersonCharacter OtherActor)
  (Variables|Default|SetCanOpen false))

(event Custom|OnBonusUIExit
  (bind _returnvalue (Game|GetPlayerController 0))
  (Widget|RemovefromParent (stale Input|EnhancedActionEvents|EnhancedInputActionIA_Interact _output_get))
  (Input|SetInputModeGameOnly _returnvalue false)
  (Variables|/Script/Engine.PlayerController|SetbShowMouseCursor _returnvalue false)
  (Variables|Default|SetBonusUIRef 0))

(event Input|EnhancedActionEvents|EnhancedInputActionIA_Interact
  (params (ActionValue :type Boolean) (ElapsedSeconds :type Float%20%28double-precision%29) (TriggeredSeconds :type Float%20%28double-precision%29) (InputAction :type Input%20Action%20Object%20Reference :default "/Game/Assets/Input/Actions/IA_Interact.IA_Interact"))
  (bind _returnvalue (Game|GetPlayerController 0))
  (if (Variables|Default|GetCanOpen)
    (Utilities|IsValid (Variables|Default|GetBonusUIRef)
      (:Is%20Not%20Valid
        (bind _returnvalue_2 (UserInterface|CreateWidget "/Game/Assets/UI/WBP_BonusSelect.WBP_BonusSelect_C" _returnvalue self))
        (bind _output_get (Variables|Default|SetBonusUIRef _returnvalue_2))
        (EventDispatchers|BindEventtoOnExitRequested _output_get (delegate Custom|OnBonusUIExit))
        (UserInterface|Viewport|AddtoViewport _output_get 0)
        (Input|SetInputModeUIOnly _returnvalue _output_get "DoNotLock" false)
        (Variables|/Script/Engine.PlayerController|SetbShowMouseCursor _returnvalue true)))))

(event EventBeginPlay
  (Input|EnableInput (Game|GetPlayerController 0)))

(event Collision|EventActorBeginOverlap
  (params (OtherActor :type Actor%20Object%20Reference)))

(event EventTick
  (params (DeltaSeconds :type Float%20%28single-precision%29)))

(fn ConstructionScript)