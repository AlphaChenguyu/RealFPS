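; Blood Pace buff that grants its third-person character owner a temporary walk-speed boost, apparently on enemy kills.
; On creation it binds to the owner's OnEnemyKilled event.
; SpeedUp caches the current MaxWalkSpeed, scales it by the buff value and starts a duration timer to restore it.
; Removal also restores the cached speed; repeat triggers overwrite that cache with the current, possibly boosted, speed.
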(event Custom|SpeedUp
  (bind _asbp_third_person_character (Utilities|Casting|CastToBP_ThirdPersonCharacter (Variables|Default|GetBuff%20Owner)))
  (Variables|Default|SetMax%20Walk%20Speed%20Ref (Variables|/Script/Engine.CharacterMovementComponent|GetMaxWalkSpeed (Variables|/Script/Engine.Character|GetCharacterMovement _asbp_third_person_character)))
  (Variables|/Script/Engine.CharacterMovementComponent|SetMaxWalkSpeed (Variables|/Script/Engine.Character|GetCharacterMovement _asbp_third_person_character) (* (Variables|/Script/Engine.CharacterMovementComponent|GetMaxWalkSpeed (Variables|/Script/Engine.Character|GetCharacterMovement _asbp_third_person_character)) (+ 1.0 (Utilities|Struct|BreakF_Buff (Variables|Default|GetBuffStructure)))))
  (Utilities|Time|SetTimerbyFunctionName 0 "Resume Speed" (Utilities|Struct|BreakF_Buff (Variables|Default|GetBuffStructure)))
  (Development|PrintString 0 "speed up"))

(event Custom|Resume%20Speed
  (bind _asbp_third_person_character (Utilities|Casting|CastToBP_ThirdPersonCharacter (Variables|Default|GetBuff%20Owner)))
  (Variables|/Script/Engine.CharacterMovementComponent|SetMaxWalkSpeed (Variables|/Script/Engine.Character|GetCharacterMovement _asbp_third_person_character) (Variables|Default|GetMax%20Walk%20Speed%20Ref))
  (Development|PrintString 0 "speed down"))

(fn BuffonCreate
  (bind _asbp_third_person_character (Utilities|Casting|CastToBP_ThirdPersonCharacter (Variables|Default|GetBuff%20Owner)))
  (EventDispatchers|BindEventtoOnEnemyKilled _asbp_third_person_character (EventDispatchers|CreateEvent :!event Custom|SpeedUp))
  (Development|PrintString 0 "create"))

(fn BuffonRemove
  (params (Remover :type Actor%20Object%20Reference))
  (bind _asbp_third_person_character (Utilities|Casting|CastToBP_ThirdPersonCharacter (Variables|Default|GetBuff%20Owner)))
  (Variables|/Script/Engine.CharacterMovementComponent|SetMaxWalkSpeed (Variables|/Script/Engine.Character|GetCharacterMovement _asbp_third_person_character) (Variables|Default|GetMax%20Walk%20Speed%20Ref))
  (Development|PrintString 0 "remove"))