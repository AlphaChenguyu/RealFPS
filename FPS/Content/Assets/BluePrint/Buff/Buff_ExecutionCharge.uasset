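; Execution Charge buff that recharges the owning third-person character's Siphon ability on enemy kills.
; On creation it binds to the character's OnEnemyKilled event, apparently to trigger RechargeSiphon, which zeroes the remaining Siphon cooldown.
; Removal only casts the owner and never unbinds; its fire-rate reset and debug print are disconnected.
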(event Custom|Recharge%20Siphon
  (bind _asbp_third_person_character (Utilities|Casting|CastToBP_ThirdPersonCharacter (Variables|Default|GetBuff%20Owner)))
  (Variables|/Game/Assets/BluePrint/BP_ThirdPersonCharacter.BP_ThirdPersonCharacter_C|SetSiphonCDRemaining _asbp_third_person_character 0.0)
  (Development|PrintString 0 "Recharged"))

(fn BuffonCreate
  (bind _asbp_third_person_character (Utilities|Casting|CastToBP_ThirdPersonCharacter (Variables|Default|GetBuff%20Owner)))
  (EventDispatchers|BindEventtoOnEnemyKilled _asbp_third_person_character (EventDispatchers|CreateEvent :!event Custom|Recharge%20Siphon))
  (Development|PrintString 0 "create"))

(fn BuffonRemove
  (params (Remover :type Actor%20Object%20Reference))
  (bind _asbp_third_person_character (Utilities|Casting|CastToBP_ThirdPersonCharacter (Variables|Default|GetBuff%20Owner))))