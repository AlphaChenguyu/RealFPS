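; Kill-chain buff that boosts the owning third-person character's rifle-style and shotgun fire rates, apparently triggered by enemy kills.
; BuffOnCreate binds to the character's OnEnemyKilled; FireRateUp divides both FireRate values by one plus BuffValue and starts a Duration timer.
; ResumeFireRate restores hard-coded defaults rather than saved values.
; BuffOnRemove only casts the owner, leaving the binding and rates untouched.
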(event Custom|FireRateUp
  (bind _buffstructure (Variables|Default|GetBuffStructure))
  (bind _buffvalue (Utilities|Struct|BreakF_Buff _buffstructure))
  (bind _asbp_third_person_character (Utilities|Casting|CastToBP_ThirdPersonCharacter (Variables|Default|GetBuff%20Owner)))
  (Variables|/Game/Assets/BluePrint/BP_ThirdPersonCharacter.BP_ThirdPersonCharacter_C|SetFireRate _asbp_third_person_character (/ (Variables|/Game/Assets/BluePrint/BP_ThirdPersonCharacter.BP_ThirdPersonCharacter_C|GetFireRate _asbp_third_person_character) (+ 1.0 _buffvalue)))
  (Variables|/Game/Assets/BluePrint/BP_ThirdPersonCharacter.BP_ThirdPersonCharacter_C|SetFireRate_shotgun _asbp_third_person_character (/ (Variables|/Game/Assets/BluePrint/BP_ThirdPersonCharacter.BP_ThirdPersonCharacter_C|GetFireRate_shotgun _asbp_third_person_character) (+ 1.0 _buffvalue)))
  (Utilities|Time|SetTimerbyFunctionName 0 "Resume FireRate" (Utilities|Struct|BreakF_Buff (Variables|Default|GetBuffStructure)))
  (Development|PrintString 0 "FireRate up"))

(event Custom|Resume%20FireRate
  (bind _asbp_third_person_character (Utilities|Casting|CastToBP_ThirdPersonCharacter (Variables|Default|GetBuff%20Owner)))
  (Variables|/Game/Assets/BluePrint/BP_ThirdPersonCharacter.BP_ThirdPersonCharacter_C|SetFireRate _asbp_third_person_character 0.13)
  (Variables|/Game/Assets/BluePrint/BP_ThirdPersonCharacter.BP_ThirdPersonCharacter_C|SetFireRate_shotgun _asbp_third_person_character 1.33)
  (Development|PrintString 0 "FireRate down"))

(fn BuffonCreate
  (bind _asbp_third_person_character (Utilities|Casting|CastToBP_ThirdPersonCharacter (Variables|Default|GetBuff%20Owner)))
  (EventDispatchers|BindEventtoOnEnemyKilled _asbp_third_person_character (EventDispatchers|CreateEvent :!event Custom|FireRateUp))
  (Development|PrintString 0 "create"))

(fn BuffonRemove
  (params (Remover :type Actor%20Object%20Reference))
  (bind _asbp_third_person_character (Utilities|Casting|CastToBP_ThirdPersonCharacter (Variables|Default|GetBuff%20Owner))))