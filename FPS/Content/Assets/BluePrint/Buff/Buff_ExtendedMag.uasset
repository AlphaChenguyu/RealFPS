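; Extended magazine buff that raises the total ammo of the owning third-person character's rifle and shotgun.
; On creation it casts the owner to BP_ThirdPersonCharacter and multiplies each weapon's TotalAmmo by one plus the buff's value.
; Removal and stack changes only print debug strings, so the increase is neither reverted nor rescaled with stacks.
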(fn BuffonCreate
  (bind _buffstructure (Variables|Default|GetBuffStructure))
  (bind _buffvalue (Utilities|Struct|BreakF_Buff _buffstructure))
  (bind _asbp_third_person_character (Utilities|Casting|CastToBP_ThirdPersonCharacter (Variables|Default|GetBuff%20Owner)))
  (Variables|/Game/Assets/BluePrint/Weapon/BP_M416.BP_M416_C|SetTotalAmmo (Variables|/Game/Assets/BluePrint/BP_ThirdPersonCharacter.BP_ThirdPersonCharacter_C|GetWeaponRifle _asbp_third_person_character) (* (Variables|/Game/Assets/BluePrint/Weapon/BP_M416.BP_M416_C|GetTotalAmmo (Variables|/Game/Assets/BluePrint/BP_ThirdPersonCharacter.BP_ThirdPersonCharacter_C|GetWeaponRifle _asbp_third_person_character)) (+ 1.0 _buffvalue)))
  (Variables|/Game/Assets/BluePrint/Weapon/BP_Peacekeeper.BP_Peacekeeper_C|SetTotal%20Ammo (Variables|/Game/Assets/BluePrint/BP_ThirdPersonCharacter.BP_ThirdPersonCharacter_C|GetWeaponShotgun _asbp_third_person_character) (* (Variables|/Game/Assets/BluePrint/Weapon/BP_Peacekeeper.BP_Peacekeeper_C|GetTotal%20Ammo (Variables|/Game/Assets/BluePrint/BP_ThirdPersonCharacter.BP_ThirdPersonCharacter_C|GetWeaponShotgun _asbp_third_person_character)) (+ 1.0 _buffvalue))))

(fn BuffonRemove
  (params (Remover :type Actor%20Object%20Reference))
  (Development|PrintString 0 "Remove"))

(fn BuffonChangeStack
  (params (ChangeStack :type Integer))
  (Development|PrintString 0 (Utilities|String|ToString(Integer) (Variables|Default|GetCurStack))))