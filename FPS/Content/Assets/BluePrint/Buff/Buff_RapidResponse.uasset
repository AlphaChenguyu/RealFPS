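; Rapid Response buff that makes the third-person player character move and reload faster.
; On creation it multiplies max walk speed by one plus the buff value, and rifle and shotgun reload speeds by a more strongly scaled factor of that value.
; Removal only prints a debug string and does not restore the modified speeds.
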(fn BuffonCreate
  (bind _buffstructure (Variables|Default|GetBuffStructure))
  (bind _buffvalue (Utilities|Struct|BreakF_Buff _buffstructure))
  (bind _returnvalue (* _buffvalue 2.5))
  (bind _returnvalue_2 (+ _returnvalue 1.0))
  (bind _asbp_third_person_character (Utilities|Casting|CastToBP_ThirdPersonCharacter (Variables|Default|GetBuff%20Owner)))
  (Variables|/Script/Engine.CharacterMovementComponent|SetMaxWalkSpeed (Variables|/Script/Engine.Character|GetCharacterMovement _asbp_third_person_character) (* (+ 1.0 _buffvalue) (Variables|/Script/Engine.CharacterMovementComponent|GetMaxWalkSpeed (Variables|/Script/Engine.Character|GetCharacterMovement _asbp_third_person_character))))
  (Variables|/Game/Assets/BluePrint/Weapon/BP_M416.BP_M416_C|SetRifleReloadSpeed (Variables|/Game/Assets/BluePrint/BP_ThirdPersonCharacter.BP_ThirdPersonCharacter_C|GetWeaponRifle _asbp_third_person_character) (* _returnvalue_2 (Variables|/Game/Assets/BluePrint/Weapon/BP_M416.BP_M416_C|GetRifleReloadSpeed (Variables|/Game/Assets/BluePrint/BP_ThirdPersonCharacter.BP_ThirdPersonCharacter_C|GetWeaponRifle _asbp_third_person_character))))
  (Variables|/Game/Assets/BluePrint/Weapon/BP_Peacekeeper.BP_Peacekeeper_C|SetShotgunReloadSpeed (Variables|/Game/Assets/BluePrint/BP_ThirdPersonCharacter.BP_ThirdPersonCharacter_C|GetWeaponShotgun _asbp_third_person_character) (* _returnvalue_2 (Variables|/Game/Assets/BluePrint/Weapon/BP_Peacekeeper.BP_Peacekeeper_C|GetShotgunReloadSpeed (Variables|/Game/Assets/BluePrint/BP_ThirdPersonCharacter.BP_ThirdPersonCharacter_C|GetWeaponShotgun _asbp_third_person_character)))))

(fn BuffonRemove
  (params (Remover :type Actor%20Object%20Reference))
  (Utilities|Casting|CastToBP_ThirdPersonCharacter (Variables|Default|GetBuff%20Owner))
  (Development|PrintString 0 "remove"))