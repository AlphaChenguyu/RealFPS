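; Rocket Booster buff that raises the rocket damage of the player character it is applied to.
; On creation it casts the buff owner to BP_ThirdPersonCharacter and multiplies its RocketDamage by one plus the buff value.
; Removal and stack changes only print debug text, so the boost is neither reverted nor scaled with stacks.
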(fn BuffonCreate
  (bind _asbp_third_person_character (Utilities|Casting|CastToBP_ThirdPersonCharacter (Variables|Default|GetBuff%20Owner)))
  (Variables|/Game/Assets/BluePrint/BP_ThirdPersonCharacter.BP_ThirdPersonCharacter_C|SetRocketDamage _asbp_third_person_character (* (Variables|/Game/Assets/BluePrint/BP_ThirdPersonCharacter.BP_ThirdPersonCharacter_C|GetRocketDamage _asbp_third_person_character) (+ 1.0 (Utilities|Struct|BreakF_Buff (Variables|Default|GetBuffStructure))))))

(fn BuffonRemove
  (params (Remover :type Actor%20Object%20Reference))
  (Development|PrintString 0 "Remove"))

(fn BuffonChangeStack
  (params (ChangeStack :type Integer))
  (Development|PrintString 0 (Utilities|String|ToString(Integer) (Variables|Default|GetCurStack))))