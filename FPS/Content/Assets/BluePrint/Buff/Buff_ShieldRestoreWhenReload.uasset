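; Buff that restores the owning third-person character's shield when they reload.
; On creation it binds to the reload events of the character's rifle and shotgun.
; RestoreShield adds the buff value to CurrentShield with no clamp.
; Removal and stack changes only print debug strings, so the reload bindings are not unbound here and stacking has no effect in this graph.
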(event Custom|Restore%20Shield
  (bind _asbp_third_person_character (Utilities|Casting|CastToBP_ThirdPersonCharacter (Variables|Default|GetBuff%20Owner)))
  (Variables|/Game/Assets/BluePrint/BP_ThirdPersonCharacter.BP_ThirdPersonCharacter_C|SetCurrentShield _asbp_third_person_character (+ (Utilities|Struct|BreakF_Buff (Variables|Default|GetBuffStructure)) (Variables|/Game/Assets/BluePrint/BP_ThirdPersonCharacter.BP_ThirdPersonCharacter_C|GetCurrentShield _asbp_third_person_character))))

(fn BuffonCreate
  (bind _asbp_third_person_character (Utilities|Casting|CastToBP_ThirdPersonCharacter (Variables|Default|GetBuff%20Owner)))
  (EventDispatchers|BindEventtoOnRifleReload (Variables|/Game/Assets/BluePrint/BP_ThirdPersonCharacter.BP_ThirdPersonCharacter_C|GetWeaponRifle _asbp_third_person_character) (EventDispatchers|CreateEvent :!event Custom|Restore%20Shield))
  (EventDispatchers|BindEventtoOnShotgunReload (Variables|/Game/Assets/BluePrint/BP_ThirdPersonCharacter.BP_ThirdPersonCharacter_C|GetWeaponShotgun _asbp_third_person_character) (EventDispatchers|CreateEvent :!event Custom|Restore%20Shield)))

(fn BuffonRemove
  (params (Remover :type Actor%20Object%20Reference))
  (Development|PrintString 0 "Remove"))

(fn BuffonChangeStack
  (params (ChangeStack :type Integer))
  (Development|PrintString 0 "Stack+1"))