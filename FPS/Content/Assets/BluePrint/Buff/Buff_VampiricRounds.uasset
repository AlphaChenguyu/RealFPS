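; Vampiric Rounds buff that heals its owning BP_ThirdPersonCharacter on enemy kills.
; On creation it binds to the owner's OnEnemyKilled event, evidently to drive RestoreHP.
; RestoreHP adds a fraction of MaxHealth set by the buff's BuffValue, capped at MaxHealth.
; Removal only prints a debug message and does not unbind the kill event.
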(event Custom|Restore%20HP
  (bind _asbp_third_person_character (Utilities|Casting|CastToBP_ThirdPersonCharacter (Variables|Default|GetBuff%20Owner)))
  (Variables|/Game/Assets/BluePrint/BP_ThirdPersonCharacter.BP_ThirdPersonCharacter_C|SetHealth _asbp_third_person_character (Math|Float|Min(Float) (+ (Variables|/Game/Assets/BluePrint/BP_ThirdPersonCharacter.BP_ThirdPersonCharacter_C|GetHealth _asbp_third_person_character) (* (Variables|/Game/Assets/BluePrint/BP_ThirdPersonCharacter.BP_ThirdPersonCharacter_C|GetMaxHealth _asbp_third_person_character) (Utilities|Struct|BreakF_Buff (Variables|Default|GetBuffStructure)))) (Variables|/Game/Assets/BluePrint/BP_ThirdPersonCharacter.BP_ThirdPersonCharacter_C|GetMaxHealth _asbp_third_person_character)))
  (Development|PrintString 0 "HP up"))

(fn BuffonCreate
  (bind _asbp_third_person_character (Utilities|Casting|CastToBP_ThirdPersonCharacter (Variables|Default|GetBuff%20Owner)))
  (EventDispatchers|BindEventtoOnEnemyKilled _asbp_third_person_character (EventDispatchers|CreateEvent :!event Custom|Restore%20HP))
  (Development|PrintString 0 "create"))

(fn BuffonRemove
  (params (Remover :type Actor%20Object%20Reference))
  (Utilities|Casting|CastToBP_ThirdPersonCharacter (Variables|Default|GetBuff%20Owner))
  (Development|PrintString 0 "remove"))