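; Actor component that manages buffs, creating them by ID from DT_BuffData and driving their lifecycle every Tick.
; New buffs wait in a queue; each tick merges them into the active list, stacking same-ID buffs up to their max and adding or refreshing duration per rule.
; It then ticks active buffs, defers expired ones to a removal list, and fires their remove callback.
; Buffs can also be removed by ID or object.
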(event EventBeginPlay)

(event EventTick
  (params (DeltaSeconds :type Float%20%28single-precision%29))
  (CallFunction|BuffsTick DeltaSeconds))

(fn AddBuff
  (params (Id :type Name) (Target :type Actor%20Object%20Reference))
  (bind _returnvalue (Utilities|GetDataTableRow "/Game/Assets/BluePrint/Buff/DT_BuffData.DT_BuffData" Id)
    (:then
      (bind _returnvalue_2 (Game|ConstructObjectfromClass (.Buff (Utilities|Struct|BreakF_Buff _returnvalue))))
      (Default|Init _returnvalue_2 _returnvalue Target)
      (Utilities|Array|Add (Variables|Default|GetWaitAddBuffs) _returnvalue_2))))

(fn RemoveBuffbyId
  (params (Id :type Name) (Remover :type Actor%20Object%20Reference))
  (bind _activebuffs_ (Variables|Default|GetActiveBuffs%20))
  (bind (_findbuff _isfind _index) (CallFunction|FindBufffromBuffsbyId Id _activebuffs_))
  (if _isfind
    (Utilities|Array|RemoveIndex (Variables|Default|GetActiveBuffs%20) _index)
    (Default|BuffonRemove _findbuff Remover)))

(fn RemoveBuffByobj
  (params (DeleteBuff :type BP%20Buff%20Base%20Object%20Reference) (Remover :type Actor%20Object%20Reference))
  (bind _returnvalue (Utilities|Array|RemoveItem (Variables|Default|GetActiveBuffs%20) DeleteBuff))
  (if _returnvalue
    (Default|BuffonRemove DeleteBuff Remover)))

(fn BuffsTick
  (params (DeltaTime :type Float%20%28double-precision%29))
  (Utilities|FlowControl|Sequence
    (:then_0
      ;[0.15 0.15 0.15 0.5] Handle Waited Buffs
      (for _array_element (Variables|Default|GetWaitAddBuffs)
        (bind _output_get (LocalVariables|SetLocalBuff _array_element))
        (if (.IsFind (CallFunction|FindBufffromBuffsbyId (Default|GetBuffId _output_get) (Variables|Default|GetActiveBuffs%20)))
          (LocalVariables|SetLocalBuff (.FindBuff (CallFunction|FindBufffromBuffsbyId (Default|GetBuffId _output_get) (Variables|Default|GetActiveBuffs%20))))
          (if (not (Default|IsMaxStack (LocalVariables|GetLocalBuff)))
            (Math|Integer|IncrementInt (Variables|/Game/Assets/BluePrint/Buff/BP_BuffBase.BP_BuffBase_C|GetCurStack (LocalVariables|GetLocalBuff))
              (:%20%20
                (Default|BuffonChangeStack (LocalVariables|GetLocalBuff) 1)
                (switch Utilities|FlowControl|Switch|SwitchonE_AddStackTimeRule (.AddStackTimeRule (Utilities|Struct|BreakF_Buff (Variables|/Game/Assets/BluePrint/Buff/BP_BuffBase.BP_BuffBase_C|GetBuffStructure (LocalVariables|GetLocalBuff))))
                  (:NewEnumerator0
                    (Default|AddDuration (LocalVariables|GetLocalBuff) (.Duration (Utilities|Struct|BreakF_Buff (Variables|/Game/Assets/BluePrint/Buff/BP_BuffBase.BP_BuffBase_C|GetBuffStructure (LocalVariables|GetLocalBuff))))))
                  (:NewEnumerator6
                    (Default|ResetDuration (LocalVariables|GetLocalBuff)))))))
          (else
            (Utilities|Array|Add (Variables|Default|GetActiveBuffs%20) (LocalVariables|GetLocalBuff))
            (Default|BuffonCreate (LocalVariables|GetLocalBuff)))))
      (Utilities|Array|Clear (Variables|Default|GetWaitAddBuffs)))
    (:then_1
      (for _array_element_2 (Variables|Default|GetActiveBuffs%20)
        (bind _istimeout (Default|BuffTick _array_element_2 DeltaTime))
        (if _istimeout
          (Utilities|Array|Add (Variables|Default|GetWaitRemoveBuffs) _array_element_2))))
    (:then_2
      (for _array_element_3 (Variables|Default|GetWaitRemoveBuffs)
        (CallFunction|RemoveBuffByobj _array_element_3 (Components|GetOwner)))
      (Utilities|Array|Clear (Variables|Default|GetWaitRemoveBuffs)))))

(fn FindBufffromBuffsbyId
  (params (Id :type Name) (Buffs :type Array%20of%20BP%20Buff%20Base%20Object%20References))
  (for (_array_element _array_index) Buffs
    (if (== (.BuffID (Utilities|Struct|BreakF_Buff (Variables|/Game/Assets/BluePrint/Buff/BP_BuffBase.BP_BuffBase_C|GetBuffStructure _array_element))) Id)
      (return _array_element true _array_index)))
  (return 0 false 0))