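; BP_BuffBase is a base buff object that holds a BuffStructure and tracks its elapsed time, remaining duration and period.
; Init seeds the timers from the structure, and BuffTick advances them through HandleTime, returning true once a non-permanent buff expires.
; Periodic buffs fire BuffOnPeriod when the period runs out, resetting it while the buff lasts.
; Damaged, hit, kill and period hooks are empty stubs, while BuffOnCreate only prints a message.
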(fn BuffonDamaged)

(fn BuffTick
  (params (DeltaTime :type Float%20%28double-precision%29))
  (|HandleTime)
  (if (and (<= (Variables|RunTimeVar|GetCurDuration) 0.0) (not (.IsPermanent (Utilities|Struct|BreakF_Buff (Variables|Default|GetBuffStructure)))))
    (if (and (<= (Variables|RunTimeVar|GetCurPeriod) 0.01) (.IsPeriod (Utilities|Struct|BreakF_Buff (Variables|Default|GetBuffStructure))))
      (CallFunction|BuffonPeriod))
    (return true)
    (elif (and (<= (Variables|RunTimeVar|GetCurPeriod) 0.01) (.IsPeriod (Utilities|Struct|BreakF_Buff (Variables|Default|GetBuffStructure))))
      (CallFunction|BuffonPeriod)
      (Variables|RunTimeVar|SetCurPeriod (.Period (Utilities|Struct|BreakF_Buff (Variables|Default|GetBuffStructure))))
      (return false))))

(fn BuffonHit)

(fn BuffonKil)

(fn BuffonPeriod)

(fn Init
  (params (Buff%20Structure :type F%20Buff%20Structure))
  (Variables|Default|SetBuffStructure Buff%20Structure)
  (Variables|RunTimeVar|SetCurDuration (.Duration (Utilities|Struct|BreakF_Buff (Variables|Default|GetBuffStructure))))
  (Variables|RunTimeVar|SetCurPeriod (.Period (Utilities|Struct|BreakF_Buff (Variables|Default|GetBuffStructure)))))

(fn GetBuffId
  (return (Utilities|Struct|BreakF_Buff (Variables|Default|GetBuffStructure))))

(fn BuffonCreate
  (Development|PrintString 0 (Variables|Default|Getmessage)))