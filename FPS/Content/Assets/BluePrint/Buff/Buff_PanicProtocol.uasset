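; Panic Protocol buff that gives the player character a chance to regain shield when damaged.
; On creation it binds an event to the owning BP_ThirdPersonCharacter's OnPlayerDamaged.
; RestoreShield has a one-in-four chance to add the buff's BuffValue to CurrentShield, without clamping.
; Removal and stack changes only print debug strings, so the damage binding is never explicitly unbound here.
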(event Custom|Restore%20Shield
  (params (Damage%20 :type Float%20%28double-precision%29) (DamageCauser%20 :type Actor%20Object%20Reference))
  (bind _asbp_third_person_character (Utilities|Casting|CastToBP_ThirdPersonCharacter (Variables|Default|GetBuff%20Owner)))
  (if (<= (Math|Random|RandomFloatinRange 0.0 1.0) 0.25)
    (Variables|/Game/Assets/BluePrint/BP_ThirdPersonCharacter.BP_ThirdPersonCharacter_C|SetCurrentShield _asbp_third_person_character (+ (Utilities|Struct|BreakF_Buff (Variables|Default|GetBuffStructure)) (Variables|/Game/Assets/BluePrint/BP_ThirdPersonCharacter.BP_ThirdPersonCharacter_C|GetCurrentShield _asbp_third_person_character)))))

(fn BuffonCreate
  (bind _asbp_third_person_character (Utilities|Casting|CastToBP_ThirdPersonCharacter (Variables|Default|GetBuff%20Owner)))
  (EventDispatchers|BindEventtoOnPlayerDamaged _asbp_third_person_character (EventDispatchers|CreateEvent :!event Custom|Restore%20Shield)))

(fn BuffonRemove
  (params (Remover :type Actor%20Object%20Reference))
  (Development|PrintString 0 "Remove"))

(fn BuffonChangeStack
  (params (ChangeStack :type Integer))
  (Development|PrintString 0 "Stack+1"))