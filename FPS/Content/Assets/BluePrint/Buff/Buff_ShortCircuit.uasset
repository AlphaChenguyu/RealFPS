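; Short Circuit buff that shortens the Rocket and Siphon cooldowns of the third-person character that owns it.
; On creation it casts the owner to BP_ThirdPersonCharacter and scales both cooldowns by one minus the buff value.
; Removal and stack changes only print debug strings, so the reduction is neither reverted on removal nor adjusted per stack.
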(fn BuffonCreate
  (bind _buffstructure (Variables|Default|GetBuffStructure))
  (bind _buffvalue (Utilities|Struct|BreakF_Buff _buffstructure))
  (bind _asbp_third_person_character (Utilities|Casting|CastToBP_ThirdPersonCharacter (Variables|Default|GetBuff%20Owner)))
  (Variables|/Game/Assets/BluePrint/BP_ThirdPersonCharacter.BP_ThirdPersonCharacter_C|SetRocketCD _asbp_third_person_character (* (Variables|/Game/Assets/BluePrint/BP_ThirdPersonCharacter.BP_ThirdPersonCharacter_C|GetRocketCD _asbp_third_person_character) (- 1.0 _buffvalue)))
  (Variables|/Game/Assets/BluePrint/BP_ThirdPersonCharacter.BP_ThirdPersonCharacter_C|SetSiphonCD _asbp_third_person_character (* (Variables|/Game/Assets/BluePrint/BP_ThirdPersonCharacter.BP_ThirdPersonCharacter_C|GetSiphonCD _asbp_third_person_character) (- 1.0 _buffvalue))))

(fn BuffonRemove
  (params (Remover :type Actor%20Object%20Reference))
  (Development|PrintString 0 "Remove"))

(fn BuffonChangeStack
  (params (ChangeStack :type Integer))
  (Development|PrintString 0 "Stack+1"))