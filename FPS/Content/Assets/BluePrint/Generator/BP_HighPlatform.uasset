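; High platform actor in the Generator set: a cylinder of random radius and height that carries an enemy turret.
; The construction script randomizes the Corner vector, then derives the mesh scale, rotation and height from it, along with the spawn point's height.
; A CylinderType enum selects a full, half or quarter cylinder mesh, and a Material variable skins it.
; On BeginPlay a coin flip spawns either a laser turret, slightly raised, or a regular turret at that point.
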(event EventBeginPlay
  (if (Math|Random|RandomBool)
    (Game|SpawnActorfromClass "/Game/Assets/Enemy/LaserTurret/BP_LaserTurret.BP_LaserTurret_C" (Math|Conversions|ToTransform(Vector) (+ "0.000000,0.000000,40.000000" (.location (Transformation|GetWorldTransform (Variables|Default|GetEnemySpawnPoint))))) "AdjustIfPossibleButAlwaysSpawn" "MultiplyWithRoot" 0 0)
    (else
      (Game|SpawnActorfromClass "/Game/Assets/Enemy/Turret/BP_Turret.BP_Turret_C" (Transformation|GetWorldTransform (Variables|Default|GetEnemySpawnPoint)) "AdjustIfPossibleButAlwaysSpawn" "MultiplyWithRoot" 0 0))))

(fn ConstructionScript
  (bind _output_get (Variables|Default|SetCorner (Math|Vector|MakeVector (Math|Random|RandomFloatinRange 1e+02 1.5e+02) 0.0 (Math|Random|RandomFloatinRange 3e+02 5e+02))))
  (Transformation|SetRelativeLocation (Variables|Default|GetEnemySpawnPoint) (Math|Vector|MakeVector 0.0 0.0 (.z (Variables|Default|GetCorner))) false false)
  ;[1 1 1] Sets the scale of the static mesh based on the 3D Widget
  (Transformation|SetWorldScale3D (Variables|Default|GetStaticMesh) (Math|Vector|MakeVector (Math|Vector|VectorLength (Math|Vector|MakeVector (.x (/ _output_get 100)) (.y (/ _output_get 100)) 0.0)) (Math|Vector|VectorLength (Math|Vector|MakeVector (.x (/ _output_get 100)) (.y (/ _output_get 100)) 0.0)) (/ (.z (/ _output_get 100)) 2.0)))
  ;[1 1 1] Sets the static mesh based on the Enum
  (Components|StaticMesh|SetStaticMesh (Variables|Default|GetStaticMesh) (Utilities|Select :Index (Variables|Default|GetCylinderType) :NewEnumerator0 "/Game/LDToolkit/Back-end/Models/SM_CylinderTool.SM_CylinderTool" :NewEnumerator1 "/Game/LDToolkit/Back-end/Models/SM_HalfCylinderTool.SM_HalfCylinderTool" :NewEnumerator2 "/Game/LDToolkit/Back-end/Models/SM_QuarterCylinderTool.SM_QuarterCylinderTool"))
  ;[1 1 1] Sets the rotation of the static mesh to fit the 3D Widget
  (Transformation|SetRelativeRotation (Variables|Default|GetStaticMesh) (Math|Rotator|MakeRotator (.roll (Math|Rotator|FindLookatRotation (Math|Vector|MakeVector 0.0 0.0 0.0) (Math|Vector|MakeVector (.x (Variables|Default|GetCorner)) (.y (Variables|Default|GetCorner)) 0.0))) (.pitch (Math|Rotator|FindLookatRotation (Math|Vector|MakeVector 0.0 0.0 0.0) (Math|Vector|MakeVector (.x (Variables|Default|GetCorner)) (.y (Variables|Default|GetCorner)) 0.0))) (+ (.yaw (Math|Rotator|FindLookatRotation (Math|Vector|MakeVector 0.0 0.0 0.0) (Math|Vector|MakeVector (.x (Variables|Default|GetCorner)) (.y (Variables|Default|GetCorner)) 0.0))) 9e+01)) false false)
  ;[1 1 1] Sets the location of the cylinder based on the 3D Widget
  (Transformation|SetRelativeLocation (Variables|Default|GetStaticMesh) (Math|Vector|MakeVector 0.0 0.0 (/ (.z (Variables|Default|GetCorner)) 2.0)) false false)
  ;[1 1 1] Set the material of the static mesh
  (Rendering|Material|SetMaterial (Variables|Default|GetStaticMesh) 0 (Variables|Default|GetMaterial)))