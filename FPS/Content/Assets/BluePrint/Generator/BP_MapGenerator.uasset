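; BP_MapGenerator is an unfinished random map generator that builds tile codes on BeginPlay.
; Nested GridSize loops append codes to TempRow through independent percentage rolls plus an unconditional final code, so one cell can add several entries.
; TempRow is never cleared or read.
; Spawn nodes for toxic pools, box tools, runnable walls and turret platforms are unconnected, so nothing is placed in the world.
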(event EventBeginPlay
  (bind _returnvalue (Math|Random|RandomIntegerinRange 0 100))
  (for _index (range 0 (- (Variables|Default|GetGridSize) 1))
    (for _index_2 (range 0 (- (Variables|Default|GetGridSize) 1))
      (Utilities|FlowControl|Sequence
        (:then_0
          (if (<= _returnvalue 10)
            (Utilities|Array|Add (Variables|Default|GetTempRow) -1)))
        (:then_1
          (if (<= _returnvalue 60)
            (Utilities|Array|Add (Variables|Default|GetTempRow) 0)))
        (:then_2
          (if (<= _returnvalue 80)
            (Utilities|Array|Add (Variables|Default|GetTempRow) 3)))
        (:then_3
          (Utilities|Array|Add (Variables|Default|GetTempRow) 5))))))

(fn ConstructionScript)