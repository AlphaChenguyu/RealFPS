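; FPS game mode that runs a wave-based enemy survival loop, starting the first wave at BeginPlay.
; Each wave spawns twice the wave number in BP_AIBase enemies, split evenly between two spawn locations.
; EnemyKilled counts down the remaining enemies, then advances the wave until MaxWaves, showing wave UI on the player character before a delayed spawn.
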(event Custom|Start%20Game
  ;[0.15 0.15 0.15 0.5] Start Game
  (CallFunction|SpawnEnemy))

(event Custom|Spawn%20Enemy
  ;[0.15 0.15 0.15 0.5] Spawn Enemy
  (bind _output_get (Variables|Default|SetEnemyTotal (* (Variables|Default|GetCurrent%20Wave) 2)))
  (Variables|Default|SetEnemyLeft _output_get)
  (bind _index (Utilities|FlowControl|ForLoopwithBreak 0 _output_get :!label _label)
    (:LoopBody
      (if (== _index (/ (Variables|Default|GetEnemyTotal) 2))
        (goto _label Break)
        (else
          (Game|SpawnActorfromClass "/Game/Assets/Enemy/Mutant/BP_AIBase.BP_AIBase_C" (Variables|Default|GetSpawn%20Location1) "Undefined" "MultiplyWithRoot" 0 0))))
    (:Completed
      (Utilities|FlowControl|ForLoopwithBreak 1 (/ (Variables|Default|GetEnemyTotal) 2)
        (:LoopBody
          (Game|SpawnActorfromClass "/Game/Assets/Enemy/Mutant/BP_AIBase.BP_AIBase_C" (Variables|Default|GetSpawn%20Location2) "Undefined" "MultiplyWithRoot" 0 0))))))

(event Custom|Enemy%20Killed
  ;[0.15 0.15 0.15 0.5] Enemy Killed
  (bind _result (Math|Integer|DecrementInt (Variables|Default|GetEnemyLeft))
    (:%20%20
      (if (== _result 0)
        (CallFunction|NewWave)))))

(event Custom|New%20Wave
  ;[0.15 0.15 0.15 0.5] Update Wave
  (if (not (== (Variables|Default|GetCurrent%20Wave) (Variables|Default|GetMaxWaves)))
    (Math|Integer|IncrementInt (Variables|Default|GetCurrent%20Wave)
      (:%20%20
        (CallFunction|WaveStart)))))

(event Custom|Wave%20Start
  ;[0.15 0.15 0.15 0.5] Start next wave
  (bind _asbp_third_person_character (Utilities|Casting|CastToBP_ThirdPersonCharacter (Game|GetPlayerCharacter 0)))
  (Default|ShowWaveUI _asbp_third_person_character (Variables|Default|GetCurrent%20Wave))
  (Utilities|FlowControl|Delay 5.0)
  (CallFunction|SpawnEnemy))

(event EventBeginPlay
  ;[0.15 0.15 0.15 0.5] Start Game
  (CallFunction|StartGame))

(fn ConstructionScript)