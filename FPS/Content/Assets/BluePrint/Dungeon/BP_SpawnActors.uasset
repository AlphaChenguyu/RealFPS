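; Dungeon spawner actor that creates instances of a configured class on BeginPlay, owned by its parent actor.
; Selection picks the mode: random positions and yaw inside BoxArea, randomly chosen SpawnPoints, or every SpawnPoint, with points offset from the box's location.
; GetRandomIndex draws non-repeating indices by re-rolling duplicates and prints them; it loops endlessly if Number exceeds the point count.
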(event EventBeginPlay
  (switch Utilities|FlowControl|Switch|SwitchonSpawnMethods (Variables|Default|GetSelection)
    (:NewEnumerator0
      (CallFunction|InArea 0 (Variables|Default|GetNumber) (Variables|Default|GetActor%20Class)))
    (:NewEnumerator1
      (CallFunction|RandomPoint (Variables|Default|GetSpawn%20Points) (Variables|Default|GetActor%20Class) (Variables|Default|GetNumber)))
    (:NewEnumerator2
      (CallFunction|FixedPoint (Variables|Default|GetSpawn%20Points) (Variables|Default|GetActor%20Class)))))

(fn ConstructionScript)

(fn InArea
  (params (SpawnArea :type Actor%20Object%20Reference) (Number :type Integer) (ActorClass :type Actor%20Class%20Reference))
  (for _index (range 1 Number)
    (Game|SpawnActorfromClass ActorClass (Math|Transform|MakeTransform (Math|Random|RandomPointinBoundingBox (Transformation|GetActorLocation) (Components|Box|GetScaledBoxExtent (Variables|Default|GetBoxArea))) (Math|Rotator|MakeRotator 0.0 0.0 (Math|Random|RandomFloatinRange 0.0 3.6e+02))) "AdjustIfPossibleButAlwaysSpawn" "MultiplyWithRoot" (Actor|GetParentActor) 0)))

(fn RandomPoint
  (params (Points :type Array%20of%20Vectors) (ActorClass :type Actor%20Class%20Reference) (Number :type Integer))
  (bind _randomints (CallFunction|GetRandomIndex Number (Utilities|Array|Length Points) false))
  (for _array_element _randomints
    (Game|SpawnActorfromClass ActorClass (Math|Transform|MakeTransform (+ (Utilities|Array|Get(acopy) Points _array_element) (Transformation|GetWorldLocation (Variables|Default|GetBoxArea))) "0, 0, 0" "1.000000,1.000000,1.000000") "AdjustIfPossibleButAlwaysSpawn" "MultiplyWithRoot" (Actor|GetParentActor) 0)))

(fn FixedPoint
  (params (SpawnPoints :type Array%20of%20Vectors) (Class :type Actor%20Class%20Reference))
  ;[0.15 0.15 0.15 0.5] 所有点均生成
  (for _array_element SpawnPoints
    (Game|SpawnActorfromClass Class (Math|Transform|MakeTransform (+ _array_element (Transformation|GetWorldLocation (Variables|Default|GetBoxArea))) "0, 0, 0" "1.000000,1.000000,1.000000") "AdjustIfPossibleButAlwaysSpawn" "MultiplyWithRoot" (Actor|GetParentActor) 0)))

(fn GetRandomIndex
  (params (IndexAmount :type Integer) (MaxIndex :type Integer) (Repeat :type Boolean))
  (if (not Repeat)
    (for _index (range 1 IndexAmount)
      (bind _output_get (LocalVariables|SetRandomInt (Math|Random|RandomInteger MaxIndex)))
      (while (Utilities|Array|ContainsItem (LocalVariables|GetRandomIntArray) _output_get)
        (LocalVariables|SetRandomInt (Math|Random|RandomInteger MaxIndex)))
      (Utilities|Array|Add (LocalVariables|GetRandomIntArray) (LocalVariables|GetRandomInt)))
    (for _array_element (LocalVariables|GetRandomIntArray)
      (Development|PrintString (Utilities|String|ToString(Integer) _array_element)))
    (return (LocalVariables|GetRandomIntArray))))