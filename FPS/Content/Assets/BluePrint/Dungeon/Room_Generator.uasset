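; Procedural dungeon generator that grows a room layout from a start room using a seeded random stream.
; Rooms attach at random exits, retrying on overlap, with the last drawn from a special list.
; It then caps open exits and spawns doors, enemies, chests and hazards.
; MainLevel3 reloads if generation times out or validation fails on room-class counts or breadth-first distance between rooms 0 and 10.
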(event Custom|SpawnStartRoom
  ;[0.15 0.15 0.15 0.5 30] SpawnStartRoom
  (bind _returnvalue (Game|SpawnActorfromClass "/Game/Assets/BluePrint/Dungeon/BP_Room_Start.BP_Room_Start_C" (Transformation|GetWorldTransform (Variables|Default|GetDefaultSceneRoot)) "AlwaysSpawn" "MultiplyWithRoot" 0 0))
  (Utilities|Array|AppendArray (Variables|Default|GetExits%20List) (Components|GetChildrenComponents (Variables|/Game/Assets/BluePrint/Dungeon/BP_Master_Room.BP_Master_Room_C|GetExitsFolder _returnvalue) false))
  (Variables|/Game/Assets/BluePrint/Dungeon/BP_Master_Room.BP_Master_Room_C|SetRoomIndex _returnvalue (Variables|IsMapValid|GetRoomCounter))
  (bind _output_get (Variables|IsMapValid|SetRoomCounter (+ 1 (Variables|IsMapValid|GetRoomCounter))))
  (Utilities|Map|Add (Variables|IsMapValid|GetRoomMap%20) _output_get _returnvalue)
  (Variables|IsMapValid|SetRoomAIndex _returnvalue))

(event Custom|SpawnNextRoom
  ;[0.15 0.15 0.15 0.5 30] SpawnNextRoom
  (Variables|Default|SetSelectedExitPoint (.OutItem (Utilities|Array|RandomFromStream (Variables|Default|GetExits%20List) (Variables|Default|GetStream))))
  (bind _returnvalue (Game|SpawnActorfromClass (.OutItem (Utilities|Array|RandomFromStream (Variables|Default|GetRoom%20List) (Variables|Default|GetStream))) (Transformation|GetWorldTransform (Variables|Default|GetSelectedExitPoint)) "AlwaysSpawn" "MultiplyWithRoot" 0 0))
  (bind _asbp_master_room (Utilities|Casting|CastToBP_Master_Room _returnvalue))
  (Variables|IsMapValid|SetLatest%20Room _asbp_master_room)
  (Utilities|FlowControl|Delay 0.01)
  (CallFunction|CheckforOverlap))

(event Custom|IsMapValid
  (bind _roomclasscounts (Variables|IsMapValid|GetRoomClassCounts))
  (bind _value (Utilities|Map|Find _roomclasscounts "/Game/Assets/BluePrint/Dungeon/BP_Room_7.BP_Room_7_C"))
  (bind _value_2 (Utilities|Map|Find _roomclasscounts "/Game/Assets/BluePrint/Dungeon/BP_Room_6.BP_Room_6_C"))
  ;[0.15 0.15 0.15 0.5] IsMapValid
  (bind _outactors (Actor|GetAllActorsOfClass "/Game/Assets/BluePrint/Dungeon/BP_Master_Room.BP_Master_Room_C"))
  (for _array_element _outactors
    (if (Utilities|Map|Contains (Variables|IsMapValid|GetRoomClassCounts) (Utilities|GetClass _array_element))
      (Utilities|Map|Add (Variables|IsMapValid|GetRoomClassCounts) (Utilities|GetClass _array_element) (+ (.Value (Utilities|Map|Find (Variables|IsMapValid|GetRoomClassCounts) (Utilities|GetClass _array_element))) 1))
      (else
        (Utilities|Map|Add (Variables|IsMapValid|GetRoomClassCounts) (Utilities|GetClass _array_element) 1))))
  (Utilities|FlowControl|Sequence
    (:then_0
      (if (> _value_2 1)
        (Variables|IsMapValid|Setroom6数量＞1 true)))
    (:then_1
      (if (> _value 1)
        (Variables|IsMapValid|Setroom7数量＞1 true)))
    (:then_2
      (if (< (+ _value _value_2) 1)
        (Variables|IsMapValid|Set没有Special%20Room%20 true)))
    (:then_3
      (if (> (.Value (Utilities|Map|Find _roomclasscounts "/Game/Assets/BluePrint/Dungeon/BP_Room_5.BP_Room_5_C")) 1)
        (Variables|IsMapValid|Setroom5数量＞1 true)))
    (:then_4
      (if (Math|Boolean|ORBoolean (Variables|IsMapValid|Getroom6数量＞1) (Variables|IsMapValid|Getroom7数量＞1) (Variables|IsMapValid|GetSB距离≤3) (Variables|IsMapValid|Get没有Special%20Room%20) (Variables|IsMapValid|Getroom5数量＞1))
        (Game|OpenLevel(byName) "MainLevel3")
        (Development|PrintString "Respawn")))))

(event Custom|Spawn%20Doors
  ;[0.15 0.15 0.15 0.5] Spawn Doors
  (for _array_element (Variables|Default|GetDoor%20List)
    (Game|SpawnActorfromClass (.OutItem (Utilities|Array|RandomFromStream (Variables|Default|GetDoor%20Actor%20List) (Variables|Default|GetStream))) (Transformation|GetWorldTransform _array_element) "AlwaysSpawn" "MultiplyWithRoot" 0 0)))

(event Custom|Spawn%20Chest%20at%20Loc
  ;[0.15 0.15 0.15 0.5] Spawn Chest at Loc
  (if (not (<= (Variables|SpawnAmount|GetChest%20Amonut) 0)) :!label _label
    (Variables|Default|SetSelectedSpawnPoint (.OutItem (Utilities|Array|RandomFromStream (Variables|Default|GetChest%20Spawn%20points%20List) (Variables|Default|GetStream))))
    (Game|SpawnActorfromClass "/Game/Assets/BluePrint/Interact/BP_Chest.BP_Chest_C" (Math|Transform|MakeTransform (Transformation|GetWorldLocation (Variables|Default|GetSelectedSpawnPoint)) "0, 0, 0" "1.000000,1.000000,1.000000") "AdjustIfPossibleButAlwaysSpawn" "MultiplyWithRoot" 0 0)
    (Utilities|Array|RemoveItem (Variables|Default|GetChest%20Spawn%20points%20List) (Variables|Default|GetSelectedSpawnPoint))
    (Variables|SpawnAmount|SetChest%20Amonut (- (Variables|SpawnAmount|GetChest%20Amonut) 1))
    (goto _label)))

(event Custom|Spawn%20ToxicPool%20at%20Loc
  ;[0.15 0.15 0.15 0.5] Spawn ToxicPool at Loc
  (if (not (<= (Variables|SpawnAmount|GetToxic%20Pool%20Amonut) 0)) :!label _label
    (Variables|Default|SetSelectedSpawnPoint (.OutItem (Utilities|Array|RandomFromStream (Variables|Default|GetTerrain%20Spawn%20points%20List) (Variables|Default|GetStream))))
    (Game|SpawnActorfromClass "/Game/Assets/BluePrint/Dungeon/BP_Random_ToxicPool.BP_Random_ToxicPool_C" (Math|Transform|MakeTransform (+ (Transformation|GetWorldLocation (Variables|Default|GetSelectedSpawnPoint)) "0.000000,0.000000,100.000000") "0, 0, 0" "1.000000,1.000000,1.000000") "AlwaysSpawn" "MultiplyWithRoot" 0 0)
    (Utilities|Array|RemoveItem (Variables|Default|GetTerrain%20Spawn%20points%20List) (Variables|Default|GetSelectedSpawnPoint))
    (Variables|SpawnAmount|SetToxic%20Pool%20Amonut (- (Variables|SpawnAmount|GetToxic%20Pool%20Amonut) 1))
    (goto _label)))

(event Custom|Spawn%20Drone%20at%20Loc
  ;[0.15 0.15 0.15 0.5] Spawn Drone at Loc
  (if (not (<= (Variables|SpawnAmount|GetDrone%20Amonut) 0)) :!label _label
    (Variables|Default|SetSelectedSpawnPoint (.OutItem (Utilities|Array|RandomFromStream (Variables|Default|GetEnemy%20Spawn%20points%20List) (Variables|Default|GetStream))))
    (Game|SpawnActorfromClass "/Game/Assets/Enemy/Drone/BP_DroneEnemy.BP_DroneEnemy_C" (Math|Transform|MakeTransform (+ (Transformation|GetWorldLocation (Variables|Default|GetSelectedSpawnPoint)) "0.000000,0.000000,700.000000") "0, 0, 0" "1.000000,1.000000,1.000000") "AdjustIfPossibleButAlwaysSpawn" "MultiplyWithRoot" 0 0)
    (Utilities|Array|RemoveItem (Variables|Default|GetEnemy%20Spawn%20points%20List) (Variables|Default|GetSelectedSpawnPoint))
    (Variables|SpawnAmount|SetDrone%20Amonut (- (Variables|SpawnAmount|GetDrone%20Amonut) 1))
    (goto _label)))

(event Custom|Spawn%20Wheeled%20at%20Loc
  ;[0.15 0.15 0.15 0.5] Spawn Wheeled at Loc
  (if (not (<= (Variables|SpawnAmount|GetWheeledAmonut) 0)) :!label _label
    (Variables|Default|SetSelectedSpawnPoint (.OutItem (Utilities|Array|RandomFromStream (Variables|Default|GetEnemy%20Spawn%20points%20List) (Variables|Default|GetStream))))
    (Game|SpawnActorfromClass "/Game/Assets/Enemy/WheeledRobot/BP_Wheeled.BP_Wheeled_C" (Math|Transform|MakeTransform (Transformation|GetWorldLocation (Variables|Default|GetSelectedSpawnPoint)) "0, 0, 0" "1.000000,1.000000,1.000000") "AdjustIfPossibleButAlwaysSpawn" "MultiplyWithRoot" 0 0)
    (Utilities|Array|RemoveItem (Variables|Default|GetEnemy%20Spawn%20points%20List) (Variables|Default|GetSelectedSpawnPoint))
    (Variables|SpawnAmount|SetWheeledAmonut (- (Variables|SpawnAmount|GetWheeledAmonut) 1))
    (goto _label)))

(event Custom|DistanceRule
  ;[0.15 0.15 0.15 0.5] Distance Rule
  (bind _valuepin (Utilities|Map|ForEachLoop(Map) (Variables|IsMapValid|GetRoomMap%20))
    (:then
      (for _array_element (Variables|/Game/Assets/BluePrint/Dungeon/BP_Master_Room.BP_Master_Room_C|GetConnectedRoomIndices _valuepin)
        (Utilities|Array|Add (Variables|IsMapValid|GetFromRooms%20) (Variables|/Game/Assets/BluePrint/Dungeon/BP_Master_Room.BP_Master_Room_C|GetRoomIndex _valuepin))
        (Utilities|Array|Add (Variables|IsMapValid|GetToRooms%20) _array_element))
      (bind _distance (CallFunction|CalculateDistance 0 10))
      (Variables|IsMapValid|SetSB距离≤3 (<= _distance 3)))))

(event Custom|Add%20Overlapping%20Rooms%20to%20List
  ;[0.15 0.15 0.15 0.5 30] Check Overlapping Rooms
  (for _array_element (Components|GetChildrenComponents (Variables|/Game/Assets/BluePrint/Dungeon/BP_Master_Room.BP_Master_Room_C|GetOverlapFolder (Variables|IsMapValid|GetLatest%20Room)) false)
    (bind _as盒体碰撞 (Utilities|Casting|CastToBoxComponent _array_element))
    (Utilities|Array|AppendArray (Variables|Default|GetOverlapped%20List) (Class|PrimitiveComponent|GetOverlappingComponents _as盒体碰撞))))

(event Custom|Spawn%20Turrets%20at%20Loc
  ;[0.15 0.15 0.15 0.5] Spawn Turrets at Loc
  (if (not (<= (Variables|SpawnAmount|GetTurret%20Amonut) 0)) :!label _label
    (Variables|Default|SetSelectedSpawnPoint (.OutItem (Utilities|Array|RandomFromStream (Variables|Default|GetEnemy%20Spawn%20points%20List) (Variables|Default|GetStream))))
    (Game|SpawnActorfromClass "/Game/Assets/BluePrint/Dungeon/BP_TurretsPlatform.BP_TurretsPlatform_C" (Math|Transform|MakeTransform (Transformation|GetWorldLocation (Variables|Default|GetSelectedSpawnPoint)) "0, 0, 0" "1.000000,1.000000,1.000000") "AdjustIfPossibleButAlwaysSpawn" "MultiplyWithRoot" 0 0)
    (Utilities|Array|RemoveItem (Variables|Default|GetEnemy%20Spawn%20points%20List) (Variables|Default|GetSelectedSpawnPoint))
    (Variables|SpawnAmount|SetTurret%20Amonut (- (Variables|SpawnAmount|GetTurret%20Amonut) 1))
    (goto _label)))

(event Custom|Check%20For%20Overlap
  (bind _latest_room (Variables|IsMapValid|GetLatest%20Room))
  (bind _selectedexitpoint (Variables|Default|GetSelectedExitPoint))
  ;[0.15 0.15 0.15 0.5 30] Delete lastest room if Overlapping
  (CallFunction|AddOverlappingRoomstoList)
  (if (Utilities|Array|IsNotEmpty (Variables|Default|GetOverlapped%20List))
    (Utilities|Array|Clear (Variables|Default|GetOverlapped%20List))
    (Actor|DestroyActor (Variables|IsMapValid|GetLatest%20Room))
    (CallFunction|SpawnNextRoom)
    (else
      (Utilities|Array|Clear (Variables|Default|GetOverlapped%20List))
      (Variables|/Game/Assets/BluePrint/Dungeon/BP_Master_Room.BP_Master_Room_C|SetRoomIndex (Variables|IsMapValid|GetLatest%20Room) (Variables|IsMapValid|GetRoomCounter))
      (bind _output_get (Variables|IsMapValid|SetRoomCounter (+ 1 (Variables|IsMapValid|GetRoomCounter))))
      (Utilities|Map|Add (Variables|IsMapValid|GetRoomMap%20) _output_get _latest_room)
      (bind _asbp_master_room (Utilities|Casting|CastToBP_Master_Room (Components|GetOwner _selectedexitpoint)))
      (bind _output_get_2 (Variables|IsMapValid|SetRoomAIndex _asbp_master_room))
      (Default|AddConnection _output_get_2 (Variables|/Game/Assets/BluePrint/Dungeon/BP_Master_Room.BP_Master_Room_C|GetRoomIndex _latest_room))
      (Default|AddConnection _latest_room (Variables|/Game/Assets/BluePrint/Dungeon/BP_Master_Room.BP_Master_Room_C|GetRoomIndex _asbp_master_room))
      (Variables|Default|SetRoomAmount (- (Variables|Default|GetRoomAmount) 1))
      (Utilities|Array|RemoveItem (Variables|Default|GetExits%20List) _selectedexitpoint)
      ;;[0.15 0.15 0.15 0.5] Add to door list
      (Utilities|Array|Add (Variables|Default|GetDoor%20List) (Variables|Default|GetSelectedExitPoint))
      (Utilities|Array|AppendArray (Variables|Default|GetExits%20List) (Components|GetChildrenComponents (Variables|/Game/Assets/BluePrint/Dungeon/BP_Master_Room.BP_Master_Room_C|GetExitsFolder (Variables|IsMapValid|GetLatest%20Room)) false))
      (CallFunction|AddSpawnPointstoList)
      (if (> (Variables|Default|GetRoomAmount) 0)
        (if (== (Variables|Default|GetRoomAmount) 1)
          (Variables|Default|SetRoom%20List (Variables|Default|GetSpecial%20Room%20List))
          (CallFunction|SpawnNextRoom)
          (else
            (Variables|Default|SetRoom%20List (Variables|Default|GetBase%20Room%20List))
            (CallFunction|SpawnNextRoom)))
        (else
          (Utilities|FlowControl|Delay 0.0)
          (CallFunction|CloseHoles)
          (CallFunction|SpawnDoors)
          (CallFunction|SpawnWheeledatLoc)
          (CallFunction|SpawnTurretsatLoc)
          (CallFunction|SpawnDroneatLoc)
          (CallFunction|SpawnChestatLoc)
          (CallFunction|SpawnToxicPoolatLoc)
          (CallFunction|SpawnDamageWallatLoc)
          (Variables|Default|SetDungeon%20Complete true)
          (CallFunction|DistanceRule)
          (CallFunction|IsMapValid)
          (Utilities|Time|ClearandInvalidateTimerbyHandle (Variables|Default|GetTimer%20Handle)))))))

(event Custom|Close%20Holes
  ;[0.15 0.15 0.15 0.5] Close Holes
  (for _array_element (Variables|Default|GetExits%20List)
    (Game|SpawnActorfromClass "/Game/Assets/BluePrint/Dungeon/BP_EndWall.BP_EndWall_C" (Transformation|GetWorldTransform _array_element) "AlwaysSpawn" "MultiplyWithRoot" 0 0)))

(event Custom|StartDTimer
  ;[0.15 0.15 0.15 0.5] Spawn Timer
  (bind _returnvalue (Utilities|Time|SetTimerbyEvent (delegate Custom|Check%20for%20Complete) 1.0 true))
  (Variables|Default|SetTimer%20Handle _returnvalue))

(event Custom|Check%20for%20Complete
  ;[0.15 0.15 0.15 0.5] Spawn Timer
  (if (>= (Utilities|Time|GetGameTimeinSeconds) 2.0)
    (Game|OpenLevel(byName) "MainLevel3")))

(event Custom|Set%20Seed
  ;[0.15 0.15 0.15 0.5] Set Seed
  (Class|KismetMathLibrary|SeedRandomStream (Variables|Default|GetStream)))

(event Custom|Add%20Spawn%20points%20to%20List
  (bind _latest_room (Variables|IsMapValid|GetLatest%20Room))
  ;[0.15 0.15 0.15 0.5] Add Spawn points to List
  (Utilities|Array|AppendArray (Variables|Default|GetChest%20Spawn%20points%20List) (Components|GetChildrenComponents (Variables|/Game/Assets/BluePrint/Dungeon/BP_Master_Room.BP_Master_Room_C|GetChest%20Spawn%20Points _latest_room) false))
  (Utilities|Array|AppendArray (Variables|Default|GetEnemy%20Spawn%20points%20List) (Components|GetChildrenComponents (Variables|/Game/Assets/BluePrint/Dungeon/BP_Master_Room.BP_Master_Room_C|GetEnemy%20Spawn%20Points _latest_room) false))
  (Utilities|Array|AppendArray (Variables|Default|GetTerrain%20Spawn%20points%20List) (Components|GetChildrenComponents (Variables|/Game/Assets/BluePrint/Dungeon/BP_Master_Room.BP_Master_Room_C|GetTerrain%20Spawn%20Points _latest_room) false))
  (Utilities|Array|AppendArray (Variables|Default|GetWall%20Spawn%20points%20List) (Components|GetChildrenComponents (Variables|/Game/Assets/BluePrint/Dungeon/BP_Master_Room.BP_Master_Room_C|GetDamage%20Wall%20Spawn%20Points _latest_room) false)))

(event Custom|Spawn%20Damage%20Wall%20at%20Loc
  ;[0.15 0.15 0.15 0.5] Spawn Damage Wall at Loc
  (if (not (<= (Variables|SpawnAmount|GetDamage%20Wall%20Amonut) 0)) :!label _label
    (Variables|Default|SetSelectedSpawnPoint (.OutItem (Utilities|Array|RandomFromStream (Variables|Default|GetWall%20Spawn%20points%20List) (Variables|Default|GetStream))))
    (Game|SpawnActorfromClass "/Game/Assets/BluePrint/Dungeon/BP_Random_DamageWallX.BP_Random_DamageWallX_C" (Transformation|GetWorldTransform (Variables|Default|GetSelectedSpawnPoint)) "AlwaysSpawn" "MultiplyWithRoot" 0 0)
    (Utilities|Array|RemoveItem (Variables|Default|GetWall%20Spawn%20points%20List) (Variables|Default|GetSelectedSpawnPoint))
    (Variables|SpawnAmount|SetDamage%20Wall%20Amonut (- (Variables|SpawnAmount|GetDamage%20Wall%20Amonut) 1))
    (goto _label)))

(event EventBeginPlay
  (CallFunction|SetSeed)
  (CallFunction|SpawnStartRoom)
  (CallFunction|StartDTimer)
  (CallFunction|SpawnNextRoom))

(fn ConstructionScript)

(fn CalculateDistance
  (params (StartRoom :type Integer) (EndRoom :type Integer))
  (Utilities|Array|Clear (LocalVariables|GetCurrentLayer%20))
  (Utilities|Array|Add (LocalVariables|GetCurrentLayer%20) StartRoom)
  (Utilities|Array|Clear (LocalVariables|GetVisited%20))
  (Utilities|Array|Add (LocalVariables|GetVisited%20) StartRoom)
  (LocalVariables|SetLayerCount%20 0)
  (while (> (Utilities|Array|Length (LocalVariables|GetCurrentLayer%20)) 0)
    (if (Utilities|Array|ContainsItem (LocalVariables|GetCurrentLayer%20) EndRoom)
      (return (LocalVariables|GetLayerCount%20))
      (else
        (Utilities|Array|Clear (LocalVariables|GetNextLayer%20))
        (bind _result (Math|Integer|IncrementInt (LocalVariables|GetLayerCount%20))
          (:%20%20
            (LocalVariables|SetLayerCount%20 _result)
            (for _array_element (LocalVariables|GetCurrentLayer%20)
              (for (_array_element_2 _array_index) (Variables|IsMapValid|GetFromRooms%20)
                (if (== _array_element_2 _array_element)
                  (if (not (Utilities|Array|ContainsItem (LocalVariables|GetVisited%20) (Utilities|Array|Get(acopy) (Variables|IsMapValid|GetToRooms%20) _array_index)))
                    (Utilities|Array|Add (LocalVariables|GetNextLayer%20) (Utilities|Array|Get(acopy) (Variables|IsMapValid|GetToRooms%20) _array_index))
                    (Utilities|Array|Add (LocalVariables|GetVisited%20) (Utilities|Array|Get(acopy) (Variables|IsMapValid|GetToRooms%20) _array_index))))))
            (LocalVariables|SetCurrentLayer%20 (LocalVariables|GetNextLayer%20)))))))
  (return -1))