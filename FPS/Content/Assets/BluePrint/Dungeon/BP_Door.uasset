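; Dungeon door that sinks when the third-person player character enters its trigger box.
; A timeline drives a Lerp on the door cube's world Z, taking X and Y from the root.
; Each timeline update also creates new blue dynamic material instances on four light cubes.
; End overlap only casts the character, so the door never closes.
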(event OnComponentBeginOverlap(Box)
  (params (OverlappedComponent :type Primitive%20Component%20Object%20Reference) (OtherActor :type Actor%20Object%20Reference) (OtherComp :type Primitive%20Component%20Object%20Reference) (OtherBodyIndex :type Integer) (bFromSweep :type Boolean) (SweepResult :type Hit%20Result%20Structure%20%28by%20ref%29))
  (bind _defaultsceneroot (Variables|Default|GetDefaultSceneRoot))
  (bind _relativelocation (Variables|/Script/Engine.SceneComponent|GetRelativeLocation _defaultsceneroot))
  (Utilities|Casting|CastToBP_ThirdPersonCharacter OtherActor)
  (bind _door_track (Timeline|时间轴 Play)
    (:Update
      (Transformation|SetWorldLocation (Variables|Default|GetCube) (Math|Vector|MakeVector (.x _relativelocation) (.y _relativelocation) (Math|Float|Lerp 0.0 -1.01e+03 _door_track)) false false)
      (CallFunction|DoorLights (Variables|Default|GetCube1))
      (CallFunction|DoorLights (Variables|Default|GetCube2))
      (CallFunction|DoorLights (Variables|Default|GetCube3))
      (CallFunction|DoorLights (Variables|Default|GetCube4)))))

(event OnComponentEndOverlap(Box)
  (params (OverlappedComponent :type Primitive%20Component%20Object%20Reference) (OtherActor :type Actor%20Object%20Reference) (OtherComp :type Primitive%20Component%20Object%20Reference) (OtherBodyIndex :type Integer))
  (Utilities|Casting|CastToBP_ThirdPersonCharacter OtherActor))

(event Custom|Door%20Lights
  (params (Door%20Light :type Primitive%20Component%20Object%20Reference))
  (Rendering|Material|CreateDynamicMaterialInstance Door%20Light 0 "/Game/Assets/Materials/M_DoorLight_Blue.M_DoorLight_Blue" "None" :!class /Script/Engine.PrimitiveComponent))

(fn ConstructionScript)