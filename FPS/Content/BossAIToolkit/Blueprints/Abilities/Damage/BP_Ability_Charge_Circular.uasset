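; Boss charge ability that moves the boss along a curved path to a point offset beyond its target.
; On BeginPlay it sets the endpoint along the boss-to-target direction and a sideways arc offset, both scaled by the ability modifier.
; Location updates blend start to end by curve X, add the offset weighted by curve Z, and apply constant-speed interpolation with sweep.
; Execution forces the boss to face the target.
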(event EventBeginPlay
  (|CallParentFunction)
  (CallFunction|SetFinalLocation))

(event EventOnExecute
  (params (Duration :type Float%20%28single-precision%29))
  (|CallParentFunction Duration)
  (CallFunction|ForceRotateAI "0, 0, 0" (Variables|Default|GetTargetActor) true))

(event EventUpdateLocation
  (params (BlendTime :type Float%20%28single-precision%29))
  (bind _curvedata (Variables|Default|GetCurveData))
  (bind _returnvalue (Math|Curves|GetVectorValue _curvedata BlendTime))
  (Transformation|SetActorLocation (Variables|Default|GetBossRef) (Math|Interpolation|VInterptoConstant (Transformation|GetActorLocation (Variables|Default|GetBossRef)) (+ (Math|Vector|Lerp(Vector) (Variables|Default|GetInitialLocation) (Variables|Default|GetFinalLocation) (.x _returnvalue)) (* (Variables|Default|GetTempAdditive) (.z _returnvalue))) (Utilities|Time|GetWorldDeltaSeconds) (Variables|Default|GetInterpSpeed)) true false))

(event EventSetFinalLocation
  (bind _bossref (Variables|Default|GetBossRef))
  (bind _targetactor (Variables|Default|GetTargetActor))
  (bind _abilityinfo (Variables|Default|GetAbilityInfo))
  (bind _modifier (Utilities|Struct|BreakF_BossAbility _abilityinfo))
  (bind _returnvalue (Transformation|GetActorLocation _targetactor))
  (bind _returnvalue_2 (Transformation|GetActorLocation _bossref))
  (bind (_x _y) (Math|Vector|BreakVector _modifier))
  (bind _returnvalue_3 (Math|Rotator|FindLookatRotation _returnvalue_2 _returnvalue))
  (Variables|Default|SetFinalLocation (+ (* (Math|Vector|GetForwardVector _returnvalue_3) _x) _returnvalue))
  (Variables|Default|SetTempAdditive (* (Math|Vector|GetRightVector _returnvalue_3) (* _y -1.0))))

(fn ConstructionScript
  (|CallParentFunction))